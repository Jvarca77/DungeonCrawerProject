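; Use rule that gates using a slotted item on its stat costs and applies those costs to the player character.
; CheckIfUseAllowed compares each of the item's CostStats against the character's current stats, failing with an "Insufficient" message naming the first stat that falls short.
; Items without costs pass, while invalid slot data fails silently.
; ResolveUseConsequence feeds CostStats into ModifyFullStats, leaving base stats unchanged.
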(fn `CheckIfUseAllowed`
  (params (Slot :type "/Game/DCT/UserInterface/WBP_Slot Object Reference"))
  (returns (bAllowed :type Boolean) (FailMessage :type String))
  (bind (_itemdata _bvalid) (`self.GetSlottedItemData` Slot))
  (if _bvalid
    (bind ((`CostStats_153_B797AEF3487A40D786043185E957F96A` _coststats)) (break `/Game/DCT/Data/FItem` _itemdata))
    (if (> (`BlueprintMapLibrary.Map_Length` _coststats) 0)
      (bind _keys (`BlueprintMapLibrary.Map_Keys` _coststats))
      (for _array_element _keys
        (if (not (>= (`BlueprintMapLibrary.Map_Find` (`/Game/DCT/Blueprints/Core/BP_PlayerCharacter.CurrentStats` (`/Game/DCT/UserInterface/WBP_Slot.PlayerCharacterRef` (`local.Slot`))) _array_element) (`BlueprintMapLibrary.Map_Find` _coststats _array_element)))
          (return false (`KismetStringLibrary.Concat_StrStr` "Insufficient " (`/Game/DCT/UserInterface/WBP_Slot.GetTagFriendlyNameFromSlot` (`local.Slot`) _array_element)))))
      (return true "")
      (else
        (return true "")))
    (else
      (return false ""))))

(fn `ResolveUseConsequence`
  (params (Slot :type "/Game/DCT/UserInterface/WBP_Slot Object Reference"))
  (returns (bSuccess :type Boolean))
  (bind _itemdata (`self.GetSlottedItemData` (`local.Slot`)))
  (bind ((`CostStats_153_B797AEF3487A40D786043185E957F96A` _coststats)) (break `/Game/DCT/Data/FItem` _itemdata))
  (if (> (`BlueprintMapLibrary.Map_Length` _coststats) 0)
    (`/Game/DCT/Blueprints/Core/BP_PlayerCharacter.ModifyFullStats` (`/Game/DCT/UserInterface/WBP_Slot.PlayerCharacterRef` (`local.Slot`)) _coststats "NewEnumerator1" false true)
    (return true)
    (else
      (return true))))