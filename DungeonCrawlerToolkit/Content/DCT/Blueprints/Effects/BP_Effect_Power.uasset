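; BP_Effect_Power is an item effect Blueprint for powers that shows the mana cost in the effect's description.
; Its GetEffectDescription override looks up Mana in the item data's CostStats and, when found, prepends the floored cost to the parent's text.
; Without a mana cost it returns the parent description unchanged.
; RunSlotEffect is an empty event, and the construction script only calls the parent.
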(event `/Game/DCT/Blueprints/Core/BPI_Interact.RunSlotEffect`
  (params (bRemoved :type Boolean) (Slot :type "/Game/DCT/UserInterface/WBP_Slot Object Reference") (SlotOwningPlayerCharacter :type "/Game/DCT/Blueprints/Core/BP_PlayerCharacter Object Reference") (ItemWidget :type "/Game/DCT/UserInterface/WBP_Item Object Reference")))

(fn `GetEffectDescription`
  (params (ItemType :type "DataTableRowHandle Structure"))
  (returns (StatDescription :type String))
  (bind (_value _returnvalue) (`BlueprintMapLibrary.Map_Find` (`.CostStats_153_B797AEF3487A40D786043185E957F96A` (break `/Game/DCT/Data/FItem` (`self.GetItemData`))) (struct :`TagName` "Stat.Mana")))
  (bind _statdescription (`parent.GetEffectDescription` ItemType))
  (if _returnvalue
    (return (`KismetStringLibrary.Concat_StrStr` " \nCost: " (`KismetStringLibrary.Conv_IntToString` (`KismetMathLibrary.FFloor` _value)) " Mana" _statdescription))
    (else
      (return _statdescription))))

(fn `UserConstructionScript`
  (`parent.UserConstructionScript`))