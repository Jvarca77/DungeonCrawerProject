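; BP_Effect_Weapon_Glowing is a slot effect that gives the player a light source tied to an item's slot.
; RunSlotEffect skips mini character slots to prevent double activation, then accepts hand and armor slot types, all sharing one branch.
; That branch adds LightProperties to the BP_LightSourceManagerComponent on player pawn 0, or removes it when the Removed flag is set.
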(event `/Game/DCT/Blueprints/Core/BPI_Interact.RunSlotEffect`
  (params (bRemoved :type Boolean) (Slot :type "/Game/DCT/UserInterface/WBP_Slot Object Reference") (SlotOwningPlayerCharacter :type "/Game/DCT/Blueprints/Core/BP_PlayerCharacter Object Reference") (ItemWidget :type "/Game/DCT/UserInterface/WBP_Item Object Reference"))
  (bind _lightproperties (`self.LightProperties`))
  (bind _returnvalue (`self.GetComponentByClass` (`GameplayStatics.GetPlayerPawn` 0) "/Game/DCT/Blueprints/Core/BP_LightSourceManagerComponent.BP_LightSourceManagerComponent_C"))
  (if (not (`/Game/DCT/UserInterface/WBP_Slot.bMiniCharacterSlot` Slot))
    (switch `/Game/DCT/Data/EItemType` (`/Game/DCT/UserInterface/WBP_Slot.SlotType` Slot)
      (:`NewEnumerator12`
        _)
      (:`NewEnumerator2`
        _)
      (:`NewEnumerator3`
        _)
      (:`NewEnumerator4`
        _)
      (:`NewEnumerator5`
        _)
      (:`NewEnumerator6`
        _)
      (:`NewEnumerator7`
        _)
      (:`NewEnumerator10`
        _))
    (if bRemoved
      (`/Game/DCT/Blueprints/Core/BP_LightSourceManagerComponent.RemoveLightSource` _returnvalue _lightproperties)
      (else
        (`/Game/DCT/Blueprints/Core/BP_LightSourceManagerComponent.AddLightSource` _returnvalue _lightproperties)))))

(fn `UserConstructionScript`
  (`parent.UserConstructionScript`))