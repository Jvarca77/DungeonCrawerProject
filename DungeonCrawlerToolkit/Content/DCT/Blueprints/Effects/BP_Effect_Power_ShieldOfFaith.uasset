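; Shield of Faith power effect that temporarily applies the item's stat bonuses to all player characters and attaches a ripple particle to the player pawn.
; A DoOnce and retriggerable delay use the item's Cooldown as duration, so reuse extends the buff without stacking it.
; Expiry or a level transition reverses the stats and destroys the emitter.
; The description override builds its text from those stats and that duration.
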(event `/Game/DCT/Blueprints/Core/BPI_Interact.UseEffect`
  (params (ActivatingPlayerCharacter :type "/Game/DCT/Blueprints/Core/BP_PlayerCharacter Object Reference") (ResidingSlot :type "/Game/DCT/UserInterface/WBP_Slot Object Reference") (ItemType :type "DataTableRowHandle Structure"))
  (`parent.UseEffect` ActivatingPlayerCharacter ResidingSlot ItemType)
  (add `/Game/DCT/Blueprints/Core/BP_GI_Dungeon.OnLevelTransition` (`.DungeonInstance` (`/Game/DCT/Blueprints/Core/BPFL_Singletons.GetDungeonGameInstance`)) (delegate `DeactivateOnTransition`))
  (`|ExecutionSequence`
    (:`then_0`
      (`/Engine/EditorBlueprintResources/StandardMacros.DoOnce` false :!label _label
        (:`Completed`
          (`self.ActivateShield`))))
    (:`then_1`
      (`KismetSystemLibrary.RetriggerableDelay` (`.Cooldown_50_6A28F6E24177E6CD22F144A81F8C2CD2` (break `/Game/DCT/Data/FItem` (`self.GetItemData`))))
      (`|ExecutionSequence`
        (:`then_0`
          (goto _label :!via `Reset`))
        (:`then_1`
          (`self.DeactivateShield`))))))

(event `ActivateShield`
  (for _array_element (`/Game/DCT/Blueprints/Core/BP_Dungeon_State.PlayerCharacters` (`.DungeonState` (`/Game/DCT/Blueprints/Core/BPFL_Singletons.GetDungeonGameState`)))
    (`/Game/DCT/Blueprints/Core/BP_PlayerCharacter.ModifyFullStats` _array_element (`.EffectStats_152_8540FAB34AD2811193CCC9A72788357A` (break `/Game/DCT/Data/FItem` (`self.GetItemData`))) "NewEnumerator0" false true))
  (bind _returnvalue (`GameplayStatics.SpawnEmitterAttached` "/Game/DCT/Particles/PS_Ripple.PS_Ripple" (`Actor.RootComponent` (`GameplayStatics.GetPlayerPawn` 0)) "None" (0.0 0.0 100.0) (struct) (1.0 1.0 0.0) "SnapToTargetIncludingScale"))
  (set `self.ShieldEmitter` _returnvalue))

(event `DeactivateOnTransition`
  (`self.DeactivateShield`))

(event `DeactivateShield`
  (remove `/Game/DCT/Blueprints/Core/BP_GI_Dungeon.OnLevelTransition` (`.DungeonInstance` (`/Game/DCT/Blueprints/Core/BPFL_Singletons.GetDungeonGameInstance`)) (delegate `DeactivateOnTransition`))
  (for _array_element (`/Game/DCT/Blueprints/Core/BP_Dungeon_State.PlayerCharacters` (`.DungeonState` (`/Game/DCT/Blueprints/Core/BPFL_Singletons.GetDungeonGameState`)))
    (`/Game/DCT/Blueprints/Core/BP_PlayerCharacter.ModifyFullStats` _array_element (`.EffectStats_152_8540FAB34AD2811193CCC9A72788357A` (break `/Game/DCT/Data/FItem` (`self.GetItemData`))) "NewEnumerator1" false true))
  (`ActorComponent.K2_DestroyComponent` (`self.ShieldEmitter`)))

(fn `GetEffectDescription`
  (params (ItemType :type "DataTableRowHandle Structure"))
  (returns (StatDescription :type String))
  (locals (LocalDescription :type String :default "Adds "))
  (bind ((`Cooldown_50_6A28F6E24177E6CD22F144A81F8C2CD2` _cooldown) (`EffectStats_152_8540FAB34AD2811193CCC9A72788357A` _effectstats)) (break `/Game/DCT/Data/FItem` (`self.GetItemData`)))
  (bind _statdescription (`parent.GetEffectDescription` ItemType))
  (bind _keys (`BlueprintMapLibrary.Map_Keys` _effectstats))
  (for (_array_element _array_index) _keys
    (bind _formattedtext (`/Game/DCT/Blueprints/Core/BPFL_Singletons.GetFormattedStatValueText` _array_element (`BlueprintMapLibrary.Map_Find` _effectstats _array_element)))
    (bind _friendlyname (`/Game/DCT/Blueprints/Core/BPFL_Singletons.GetTagFriendlyName` _array_element))
    (set `local.LocalDescription` (`KismetStringLibrary.Concat_StrStr` (`KismetMathLibrary.SelectString` (`KismetStringLibrary.Concat_StrStr` (`local.LocalDescription`) ", ") (`local.LocalDescription`) (> _array_index 0)) (`KismetTextLibrary.Conv_TextToString` _formattedtext) " " _friendlyname)))
  (return (`KismetStringLibrary.Concat_StrStr` (`KismetStringLibrary.Concat_StrStr` (`local.LocalDescription`) " to all characters. \nDuration:  " (`KismetStringLibrary.Conv_IntToString` (`KismetMathLibrary.FFloor` _cooldown)) "s") _statdescription)))

(fn `UserConstructionScript`
  (`parent.UserConstructionScript`))