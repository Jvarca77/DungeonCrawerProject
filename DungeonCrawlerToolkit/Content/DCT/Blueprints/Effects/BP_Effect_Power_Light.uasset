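; BP_Effect_Power_Light is an item effect that shines a bright light from the player for the item's Cooldown duration.
; UseEffect adds LightProperties to the player pawn's BP_LightSourceManagerComponent through a DoOnce, while a RetriggerableDelay lets repeat uses extend the light without stacking.
; Expiry or a dungeon level transition removes the light and unbinds the transition event.
; GetEffectDescription prepends the duration text to the parent description.
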(event `ActivateLight`
  (`/Game/DCT/Blueprints/Core/BP_LightSourceManagerComponent.AddLightSource` (`self.GetComponentByClass` (`GameplayStatics.GetPlayerPawn` 0) "/Game/DCT/Blueprints/Core/BP_LightSourceManagerComponent.BP_LightSourceManagerComponent_C") (`self.LightProperties`)))

(event `self.UseEffect`
  (params (ActivatingPlayerCharacter :type "/Game/DCT/Blueprints/Core/BP_PlayerCharacter Object Reference") (ResidingSlot :type "/Game/DCT/UserInterface/WBP_Slot Object Reference") (ItemType :type "DataTableRowHandle Structure"))
  (`parent.UseEffect` ActivatingPlayerCharacter ResidingSlot ItemType)
  (add `/Game/DCT/Blueprints/Core/BP_GI_Dungeon.OnLevelTransition` (`.DungeonInstance` (`/Game/DCT/Blueprints/Core/BPFL_Singletons.GetDungeonGameInstance`)) (delegate `DeactivateOnTransition`))
  (`|ExecutionSequence`
    (:`then_0`
      (`/Engine/EditorBlueprintResources/StandardMacros.DoOnce` false :!label _label
        (:`Completed`
          (`self.ActivateLight`))))
    (:`then_1`
      (`KismetSystemLibrary.RetriggerableDelay` (`.Cooldown_50_6A28F6E24177E6CD22F144A81F8C2CD2` (break `/Game/DCT/Data/FItem` (`self.GetItemData`))))
      (`|ExecutionSequence`
        (:`then_0`
          (goto _label :!via `Reset`))
        (:`then_1`
          (`self.DeactivateLight`))))))

(event `DeactivateOnTransition`
  (`self.DeactivateLight`))

(event `DeactivateLight`
  (remove `/Game/DCT/Blueprints/Core/BP_GI_Dungeon.OnLevelTransition` (`.DungeonInstance` (`/Game/DCT/Blueprints/Core/BPFL_Singletons.GetDungeonGameInstance`)) (delegate `DeactivateOnTransition`))
  (`/Game/DCT/Blueprints/Core/BP_LightSourceManagerComponent.RemoveLightSource` (`self.GetComponentByClass` (`GameplayStatics.GetPlayerPawn` 0) "/Game/DCT/Blueprints/Core/BP_LightSourceManagerComponent.BP_LightSourceManagerComponent_C") (`self.LightProperties`)))

(fn `GetEffectDescription`
  (params (ItemType :type "DataTableRowHandle Structure"))
  (returns (StatDescription :type String))
  (locals (LocalDescription :type String :default "Shines a bright light for "))
  (bind _statdescription (`parent.GetEffectDescription` ItemType))
  (return (`KismetStringLibrary.Concat_StrStr` (`KismetStringLibrary.Concat_StrStr` "Shines a bright light for " (`KismetStringLibrary.Conv_IntToString` (`KismetMathLibrary.FFloor` (`.Cooldown_50_6A28F6E24177E6CD22F144A81F8C2CD2` (break `/Game/DCT/Data/FItem` (`self.GetItemData`))))) "s") _statdescription)))

(fn `UserConstructionScript`
  (`parent.UserConstructionScript`))