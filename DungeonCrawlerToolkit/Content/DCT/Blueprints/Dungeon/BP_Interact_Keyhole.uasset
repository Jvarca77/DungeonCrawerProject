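; Dungeon keyhole interactable that powers other actors when the player uses the matching key on it.
; Interaction is allowed only if the parent check passes and the player's mouse-follow item has the required key's row name.
; Interacting clears that held item, sends a power state chosen by ReversedPower, and plays a switch sound.
; The construction script copies the key mesh's material from its data table row onto the lock mesh.
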(event `/Game/DCT/Blueprints/Core/BPI_Interact.Interact`
  (params (TriggeringActor :type "Actor Object Reference"))
  (`/Game/DCT/Blueprints/Core/BP_PC_Dungeon.ClearMouseFollowWidget` (`.DungeonPlayerController` (`/Game/DCT/Blueprints/Core/BPFL_Singletons.GetDungeonPlayerController`)))
  (`self.PowerActors` (select `bool` (`self.bReversedPower`) :`false` "NewEnumerator2" :`true` "NewEnumerator0" :!type "/Game/DCT/Data/EInteractState Enum"))
  (`GameplayStatics.PlaySoundAtLocation` "/Game/DCT/Sound/A_Switch.A_Switch" (`self.K2_GetActorLocation`) (struct) 1.0 1.0 0.0 "/Game/DCT/Sound/ATT_Dungeon.ATT_Dungeon" null null null))

(fn `CheckIfAllowedInteract`
  (params (TriggeringActor :type "Actor Object Reference"))
  (returns (bAllowed :type Boolean))
  (bind (_requiredkey_datatable _requiredkey_rowname) (break `DataTableRowHandle` (`self.RequiredKey`)))
  (bind (_itemtype_datatable _itemtype_rowname) (break `DataTableRowHandle` (`/Game/DCT/UserInterface/WBP_Item.ItemType` (`/Game/DCT/Blueprints/Core/BP_PC_Dungeon.MouseFollowWidget` (`.DungeonPlayerController` (`/Game/DCT/Blueprints/Core/BPFL_Singletons.GetDungeonPlayerController`))))))
  (bind _ballowed (`parent.CheckIfAllowedInteract` TriggeringActor))
  (if (and _ballowed (`KismetSystemLibrary.IsValid` (`/Game/DCT/Blueprints/Core/BP_PC_Dungeon.MouseFollowWidget` (`.DungeonPlayerController` (`/Game/DCT/Blueprints/Core/BPFL_Singletons.GetDungeonPlayerController`)))))
    (return (== _requiredkey_rowname _itemtype_rowname))
    (else
      (return false))))

(fn `UserConstructionScript`
  (bind (_requiredkey_datatable _requiredkey_rowname) (break `DataTableRowHandle` (`self.RequiredKey`)))
  (`parent.UserConstructionScript`)
  (bind _returnvalue (`|GetDataTableRow` _requiredkey_datatable _requiredkey_rowname)
    (:`then`
      (`PrimitiveComponent.SetMaterial` (`self.LockMesh`) 1 (`StaticMesh.GetMaterial` (`.Mesh_2_6F0C25CE46B97FD1B33001B61D51D98A` (break `/Game/DCT/Data/FItem` _returnvalue)) 0)))))