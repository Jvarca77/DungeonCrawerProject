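; Dungeon level-transition trigger that moves the game to TargetLevel when a pawn overlaps it.
; A gate opened shortly after BeginPlay passes overlaps through only if a target level is set.
; It then disables player input, fades to black, notifies and saves the DungeonInstance, stores TransitionTarget there and opens the level.
; The construction script places ExitArrow at ExitTransform.
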(event `self.ReceiveBeginPlay`
  (`KismetSystemLibrary.Delay` 0.2)
  (goto _label :!via `Open`))

(event `self.ReceiveActorBeginOverlap`
  (params (OtherActor :type "Actor Object Reference"))
  (cast `Pawn` OtherActor)
  (if (!= (`self.TargetLevel`) "None")
    (`/Engine/EditorBlueprintResources/StandardMacros.Gate` true :!label _label
      (:`Exit`
        (`self.DisableInput` (`GameplayStatics.GetPlayerPawn` 0) (`GameplayStatics.GetPlayerController` 0))
        (`PlayerCameraManager.StartCameraFade` :`self` (`GameplayStatics.GetPlayerCameraManager` 0) :`ToAlpha` 1.0 :`Duration` 0.2 :`bHoldWhenFinished` true)
        (`KismetSystemLibrary.Delay` 0.2)
        (`/Game/DCT/Blueprints/Core/BP_GI_Dungeon.OnLevelTransition` (`.DungeonInstance` (`/Game/DCT/Blueprints/Core/BPFL_Singletons.GetDungeonGameInstance`)))
        (`/Game/DCT/Blueprints/Core/BP_GI_Dungeon.SaveAll` (`.DungeonInstance` (`/Game/DCT/Blueprints/Core/BPFL_Singletons.GetDungeonGameInstance`)) false)
        (set `/Game/DCT/Blueprints/Core/BP_GI_Dungeon.TransitionTarget` (`self.TransitionTarget`) (`.DungeonInstance` (`/Game/DCT/Blueprints/Core/BPFL_Singletons.GetDungeonGameInstance`)))
        (`GameplayStatics.OpenLevel` (`self.TargetLevel`))))))

(fn `UserConstructionScript`
  (`parent.UserConstructionScript`)
  (`SceneComponent.K2_SetRelativeTransform` (`self.ExitArrow`) (`self.ExitTransform`) false false))