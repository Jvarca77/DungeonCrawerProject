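; Dungeon pressure plate that powers other actors while the weight resting on it meets a threshold.
; Overlap events sum weights from overlapping actors' GetWeightMessage to trigger Interact or release, unless the plate is exhausted.
; Power moves the plate by timeline, or snaps it when the dungeon pawn uses InstantMovement, with a switch sound and PowerActors call.
; Timed release is skipped while a BP_Effect overlaps the plate.
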(event `self.ReceiveActorBeginOverlap`
  (params (OtherActor :type "Actor Object Reference"))
  (if (`self.CheckIfExhausted`)
    _
    (elif (`|EnumEquality` (`self.InteractState`) "NewEnumerator0")
      (bind _weight (message `/Game/DCT/Blueprints/Core/BPI_Weight.GetWeight` OtherActor))
      (if (> _weight 0.0)
        (if (>= (`self.GetTotalWeightOfOverlappingObjects`) (`self.WeightThreshold`))
          (`self.Interact` OtherActor))))))

(event `self.ReceiveActorEndOverlap`
  (params (OtherActor :type "Actor Object Reference"))
  (if (`self.CheckIfExhausted`)
    _
    (elif (`|EnumEquality` (`self.InteractState`) "NewEnumerator2")
      (if (< (`self.GetTotalWeightOfOverlappingObjects`) (`self.WeightThreshold`))
        (`self.Power` null)))))

(event `self.Power`
  (params (TriggeringActor :type "Actor Object Reference") (DesiredState :type "/Game/DCT/Data/EInteractState Enum" :default "NewEnumerator0"))
  (set `self.DesiredState` DesiredState)
  (if (`/Game/DCT/Blueprints/Core/BP_DungeonPawn.bInstantMovement` (`.DungeonPawn` (`/Game/DCT/Blueprints/Core/BPFL_Singletons.GetDungeonPawn`)))
    (`SceneComponent.K2_SetRelativeLocation` (`self.Plate`) (`KismetMathLibrary.MakeVector` 0.0 0.0 (select `/Game/DCT/Data/EInteractState` (`self.DesiredState`) :`NewEnumerator2` -5.0)) false false)
    (`GameplayStatics.PlaySoundAtLocation` "/Game/DCT/Sound/A_Switch.A_Switch" (`self.K2_GetActorLocation`) (struct) 1.0 1.0 0.0 "/Game/DCT/Sound/ATT_Dungeon.ATT_Dungeon" null null null :!label _label)
    (bind _output_get (set `self.InteractState` (`self.DesiredState`)))
    (`self.PowerActors` _output_get)
    (else
      (switch `/Game/DCT/Data/EInteractState` (`self.DesiredState`)
        (:`NewEnumerator0`
          (if (== (`KismetArrayLibrary.Array_Length` (`self.GetOverlappingActors` "/Game/DCT/Blueprints/Effects/BP_Effect.BP_Effect_C")) 0)
            (bind (_direction _trigger) (`Timeline|TL_Open` :`NewTime` (select `/Game/DCT/Data/EInteractState` (stale `self.UpdateStateInstantly` DesiredState) :`NewEnumerator2` (`TimelineComponent.GetTimelineLength` (`self.TL_Open`)) :!type "Float (double-precision)") :!via `Reverse` :!label _label_2)
              (:`Update`
                (`SceneComponent.K2_SetRelativeLocation` (`self.Plate`) (`KismetMathLibrary.MakeVector` 0.0 0.0 (* _trigger -5.0)) false false))
              (:`Pressed`
                (goto _label)))))
        (:`NewEnumerator2`
          (goto _label_2))))))

(event `self.UpdateStateInstantly`
  (params (DesiredState :type "/Game/DCT/Data/EInteractState Enum" :default "NewEnumerator0"))
  (goto _label_2 :!via `SetNewTime`))

(fn `GetTotalWeightOfOverlappingObjects`
  (returns (TotalWeight :type "Float (double-precision)"))
  (locals (LocalWeight :type "Float (double-precision)"))
  (for _array_element (`self.GetOverlappingActors` null)
    (bind _weight (message `/Game/DCT/Blueprints/Core/BPI_Weight.GetWeight` _array_element))
    (if (> _weight 0.0)
      (set `local.LocalWeight` (+ (`local.LocalWeight`) _weight))))
  (return (`local.LocalWeight`)))

(fn `UserConstructionScript`)