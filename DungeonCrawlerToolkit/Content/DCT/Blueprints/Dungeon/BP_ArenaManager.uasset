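; Runs a wave-based arena, started when an interactable powers it and alerting all monsters every two seconds.
; Each wave shows a title and recursively spawns delayed monsters from DT_ArenaWaves at random spawners.
; A gate holds kill checks until spawning ends, then re-arms the interactable once all are dead, or auto-advances if none remain.
; A missing wave row powers actors, resets the dungeon save ID and opens CharacterCreation.
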(event `/Game/DCT/Blueprints/Core/BPI_Interact.Power`
  (params (TriggeringActor :type "Actor Object Reference") (DesiredState :type "/Game/DCT/Data/EInteractState Enum" :default "NewEnumerator0"))
  (if (`|EnumEquality` DesiredState "NewEnumerator2")
    (bind _asbp_interact (cast `/Game/DCT/Blueprints/Dungeon/BP_Interact` TriggeringActor))
    (set `self.TriggeringInteractable` _asbp_interact)
    (`|ExecutionSequence`
      (:`then_0`
        (`/Engine/EditorBlueprintResources/StandardMacros.DoOnce` false
          (:`Completed`
            (`self.StartAlertLoop`))))
      (:`then_1`
        (set `self.Wave` (+ (`self.Wave`) 1))
        (`self.StartNewWave` (`self.Wave`))
        (set `/Game/DCT/Blueprints/Dungeon/BP_Interact.bSingleUse` true (`self.TriggeringInteractable`))))))

(event `StartAlertLoop`
  (`KismetSystemLibrary.Delay` 2.0 :!label _label)
  (bind _outactors (`GameplayStatics.GetAllActorsOfClass` "/Game/DCT/Blueprints/Monsters/BP_Monster.BP_Monster_C"))
  (for _array_element _outactors
    (`/Game/DCT/Blueprints/Monsters/BP_Monster.Alert` _array_element))
  (goto _label))

(event `StartNewWave`
  (params (Wave :type Integer))
  (set `self.Wave` Wave)
  (set `self.WaveProgression` 0)
  (bind _returnvalue (`|CreateWidget` "/Game/DCT/UserInterface/WBP_WaveText.WBP_WaveText_C" null (select `int` (`self.Wave`) :`0` "WAVE ZERO?" :`1` "WAVE ONE" :`2` "WAVE TWO" :`3` "FINAL WAVE" :`4` "VICTORY!" :!type "Text")))
  (`UserWidget.AddToViewport` _returnvalue 0)
  (`self.AdvanceCurrentWave` 0))

(event `AdvanceCurrentWave`
  (params (WaveProgression :type Integer))
  (bind (_bvalid _dungeoninstance) (`/Game/DCT/Blueprints/Core/BPFL_Singletons.GetDungeonGameInstance`))
  (bind _triggeringinteractable (`self.TriggeringInteractable`))
  (set `self.WaveProgression` WaveProgression)
  (bind _returnvalue (`|GetDataTableRow` "/Game/DCT/Data/DT_ArenaWaves.DT_ArenaWaves" (`KismetStringLibrary.Conv_StringToName` (`KismetStringLibrary.Conv_IntToString` (`self.Wave`))))
    (:`then`
      (bind (_monsterspawnorder _spawndelays) (break `/Game/DCT/Data/FArenaWaves` _returnvalue))
      (if (< (`self.WaveProgression`) (`KismetArrayLibrary.Array_Length` _monsterspawnorder))
        (`KismetSystemLibrary.Delay` (`|GetArrayItem` _spawndelays (mod (`self.WaveProgression`) (`KismetArrayLibrary.Array_Length` _spawndelays))))
        (bind _outactors (`GameplayStatics.GetAllActorsOfClass` "/Game/DCT/Blueprints/Monsters/BP_MonsterSpawner.BP_MonsterSpawner_C"))
        (bind _returnvalue_2 (`|SpawnActorFromClass` :`Class` "/Game/DCT/Blueprints/Monsters/BP_Monster.BP_Monster_C" :`SpawnTransform` (`self.GetTransform` (`.RandomElement` (`/Game/DCT/Blueprints/Core/BPML_Utility.GetRandomElementFromArray` _outactors))) :`CollisionHandlingOverride` "Undefined" :`TransformScaleMethod` "OverrideRootScale" :`MonsterType` (`|GetArrayItem` _monsterspawnorder (`self.WaveProgression`)) :`Instigator` null))
        (add `/Game/DCT/Blueprints/Monsters/BP_Monster.OnMonsterKilled` _returnvalue_2 (delegate `KeepTrackOfKilledMonsters`))
        (`/Engine/EditorBlueprintResources/StandardMacros.IncrementInt` (`self.ActiveMonsters`)
          (:`  `
            (`self.AdvanceCurrentWave` (+ (`self.WaveProgression`) 1))))
        (elif (== (`self.ActiveMonsters`) 0)
          (`/Engine/EditorBlueprintResources/StandardMacros.IncrementInt` (`self.Wave`)
            (:`  `
              (`self.StartNewWave` (`self.Wave`))))
          (else
            (goto _label_2 :!via `Open`)))))
    (:`RowNotFound`
      (`KismetSystemLibrary.Delay` 3.0)
      (`self.PowerActors` "NewEnumerator0")
      (`/Game/DCT/Blueprints/Core/BP_GI_Dungeon.SetRandomSaveId` _dungeoninstance)
      (set `/Game/DCT/Blueprints/Core/BP_GI_Dungeon.TransitionTarget` "None" _dungeoninstance)
      (`GameplayStatics.OpenLevelBySoftObjectPtr` "/Game/DCT/Maps/CharacterCreation.CharacterCreation"))))

(event `KeepTrackOfKilledMonsters`
  (bind _triggeringinteractable (`self.TriggeringInteractable`))
  (`/Engine/EditorBlueprintResources/StandardMacros.DecrementInt` (`self.ActiveMonsters`)
    (:`  `
      (`/Engine/EditorBlueprintResources/StandardMacros.Gate` true :!label _label_2
        (:`Exit`
          (if (<= (`self.ActiveMonsters`) 0)
            (set `/Game/DCT/Blueprints/Dungeon/BP_Interact.bSingleUse` false _triggeringinteractable)
            (`self.Power` _triggeringinteractable self "NewEnumerator0")
            (bind _returnvalue (`|CreateWidget` "/Game/DCT/UserInterface/WBP_WaveText.WBP_WaveText_C" null "WAVE COMPLETE"))
            (`UserWidget.AddToViewport` _returnvalue 0)
            (goto _label_2 :!via `Close`)))))))

(fn `AttemptInteract`
  (params (TriggeringActor :type "Actor Object Reference"))
  (returns (bSuccess :type Boolean))
  (return false))

(fn `GetAttachSlot`
  (returns (AttachSlot :type "SceneComponent Object Reference"))
  (return null))

(fn `UserConstructionScript`)