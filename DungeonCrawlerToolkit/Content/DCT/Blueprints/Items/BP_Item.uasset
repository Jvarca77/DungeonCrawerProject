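; BP_Item is a world pickup for the dungeon game, with mesh and weight read from its ItemType data table row.
; While hovered, a delayed loop rechecks interaction permission and toggles rimlight on dynamic materials.
; Interaction requires the pawn's grid location within range and no existing mouse widget, then swaps the actor for a mouse-held WBP_Item.
; It saves itself to the DungeonInstance and destroys itself on UpdatePreplaced.
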(event `self.ReceiveBeginPlay`
  (for (_array_element _array_index) (`MeshComponent.GetMaterials` (`self.ItemMesh`))
    (bind _returnvalue (`PrimitiveComponent.CreateDynamicMaterialInstance` (`self.ItemMesh`) _array_index _array_element "None"))
    (`KismetArrayLibrary.Array_Add` (`self.DynamicMaterials`) _returnvalue)))

(event `self.ReceiveActorBeginCursorOver`
  (if (`self.bEnableHighlight`)
    (set `self.bCursorOver` true)
    (`/Game/DCT/Blueprints/Core/BPML_Utility.WhileLoop_Delayed` (`self.bCursorOver`) 0.1
      (:`Loop Body`
        (bind _ballowed (`self.CheckIfAllowedInteract` (`GameplayStatics.GetPlayerPawn` 0)))
        (if (!= _ballowed (`self.bHighlighted`))
          (`self.Highlight` _ballowed))))))

(event `Highlight`
  (params (bEnable :type Boolean))
  (set `self.bHighlighted` bEnable)
  (for _array_element (`self.DynamicMaterials`)
    (`MaterialInstanceDynamic.SetScalarParameterValue` _array_element "RimlightStrength" (`KismetMathLibrary.Conv_BoolToDouble` (`self.bHighlighted`)))))

(event `self.ReceiveActorEndCursorOver`
  (if (`self.bEnableHighlight`)
    (set `self.bCursorOver` false)
    (`self.Highlight` false)))

(event `self.Interact`
  (params (TriggeringActor :type "Actor Object Reference"))
  (bind _asbp_pc_dungeon (cast `/Game/DCT/Blueprints/Core/BP_PC_Dungeon` (`GameplayStatics.GetPlayerController` 0)))
  (bind _returnvalue (`|CreateWidget` "/Game/DCT/UserInterface/WBP_Item.WBP_Item_C" _asbp_pc_dungeon (`self.Amount`) (`self.ItemType`)))
  (message `/Game/DCT/Blueprints/Core/BPI_PlayerController.SetMouseWidget` (`GameplayStatics.GetPlayerController` 0) _returnvalue)
  (`self.K2_DestroyActor`))

(event `/Game/DCT/Blueprints/Core/BPI_Saveable.SaveActor`
  (params (DungeonInstance :type "/Game/DCT/Blueprints/Core/BP_GI_Dungeon Object Reference"))
  (`KismetArrayLibrary.Array_Add` (`/Game/DCT/Blueprints/Core/BP_GI_Dungeon.SavedItems` DungeonInstance) (make `/Game/DCT/Data/FItemSave` (`self.ItemType`) (`self.Amount`) (`self.GetTransform`) (`self.bEnablePhysics`))))

(event `/Game/DCT/Blueprints/Core/BPI_Saveable.UpdatePreplaced`
  (`self.K2_DestroyActor`))

(fn `AttemptInteract`
  (params (TriggeringActor :type "Actor Object Reference"))
  (returns (bSuccess :type Boolean))
  (bind _ballowed (`self.CheckIfAllowedInteract` TriggeringActor))
  (if _ballowed
    (`self.Interact` (`local.TriggeringActor`))
    (return true)
    (else
      (return false))))

(fn `CheckIfAllowedInteract`
  (params (TriggeringActor :type "Actor Object Reference"))
  (returns (bAllowed :type Boolean))
  (locals (LocalTriggeringLocation :type "Vector Structure" :default (0.0 0.0 0.0)))
  (bind _asbp_dungeon_pawn (cast `/Game/DCT/Blueprints/Core/BP_DungeonPawn` TriggeringActor))
  (bind (_value _returnvalue) (`BlueprintMapLibrary.Map_Find` (`/Game/DCT/Blueprints/Core/BP_DungeonManager.GridLocations` (`.DungeonManager` (`/Game/DCT/Blueprints/Core/BPFL_Singletons.GetDungeonManager`))) (`/Game/DCT/Blueprints/Core/BP_DungeonPawn.GridIndex` _asbp_dungeon_pawn)))
  (if _returnvalue
    (set `local.LocalTriggeringLocation` _value)
    (else
      (set `local.LocalTriggeringLocation` (`self.K2_GetActorLocation` (`local.TriggeringActor`)))))
  (if (<= (`KismetMathLibrary.Abs` (`KismetMathLibrary.Vector_Distance` (`local.LocalTriggeringLocation`) (`self.K2_GetActorLocation`))) (`/Game/DCT/Blueprints/Core/BP_DungeonManager.MaxInteractionRange` (`.DungeonManager` (`/Game/DCT/Blueprints/Core/BPFL_Singletons.GetDungeonManager`))))
    (bind _asbp_pc_dungeon (cast `/Game/DCT/Blueprints/Core/BP_PC_Dungeon` (`GameplayStatics.GetPlayerController` 0))
      (:`then`
        (`/Engine/EditorBlueprintResources/StandardMacros.IsValid` (`/Game/DCT/Blueprints/Core/BP_PC_Dungeon.MouseFollowWidget` _asbp_pc_dungeon)
          (:`Is Valid`
            (return false))
          (:`Is Not Valid`
            (return true))))
      (:`CastFailed`
        _)))
  (return false))

(fn `GetAttachSlot`
  (returns (AttachSlot :type "SceneComponent Object Reference"))
  (return null))

(fn `GetItemData`
  (returns (ItemData :type "/Game/DCT/Data/FItem Structure"))
  (bind (_itemtype_datatable _itemtype_rowname) (break `DataTableRowHandle` (`self.ItemType`)))
  (bind _returnvalue (`|GetDataTableRow` _itemtype_datatable _itemtype_rowname)
    (:`then`
      (return _returnvalue))
    (:`RowNotFound`
      (return))))

(fn `GetItemName`
  (returns (ItemName :type Name))
  (return (`.RowName` (break `DataTableRowHandle` (`self.ItemType`)))))

(fn `GetWeight`
  (returns (Weight :type "Float (double-precision)"))
  (return (`.Weight_150_32D980BD4FDFAEA5C0157FAA8AA68481` (break `/Game/DCT/Data/FItem` (`self.GetItemData`)))))

(fn `UserConstructionScript`
  (bind (_itemtype_datatable _itemtype_rowname) (break `DataTableRowHandle` (`self.ItemType`)))
  (bind _returnvalue (`|GetDataTableRow` _itemtype_datatable _itemtype_rowname)
    (:`then`
      (`StaticMeshComponent.SetStaticMesh` (`self.ItemMesh`) (`.Mesh_2_6F0C25CE46B97FD1B33001B61D51D98A` (break `/Game/DCT/Data/FItem` _returnvalue)))
      (`PrimitiveComponent.SetSimulatePhysics` (`self.ItemMesh`) (`self.bEnablePhysics`)))))