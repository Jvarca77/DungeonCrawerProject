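; BP_Projectile is a projectile that carries a held item and applies that item's effect to what it hits.
; It sweeps forward each tick with velocity and acceleration, exploding on blocking hit, non-source overlap or lifetime expiry.
; Contacts other than the source actor route through DungeonState to the item effect's ProjectileHit.
; Mesh and body particle are set at construction, with emitters and sounds for launch and impact.
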(event `self.ReceiveBeginPlay`
  (bind (_returnvalue_location _returnvalue_rotation _returnvalue_scale) (`KismetMathLibrary.BreakTransform` (`self.GetTransform`)))
  (`GameplayStatics.SpawnEmitterAtLocation` (`self.LaunchEmitter`) _returnvalue_location _returnvalue_rotation _returnvalue_scale)
  (`GameplayStatics.PlaySoundAtLocation` (`self.LaunchSound`) (`self.K2_GetActorLocation`) (struct) 1.0 1.0 0.0 "/Game/DCT/Sound/ATT_Dungeon.ATT_Dungeon" null null)
  (`KismetSystemLibrary.Delay` (`self.Lifetime`))
  (`self.Explode`))

(event `self.ReceiveTick`
  (params (DeltaSeconds :type "Float (single-precision)"))
  (`self.K2_AddActorWorldOffset` (* (`self.GetActorForwardVector`) (* (`self.Velocity`) (`GameplayStatics.GetWorldDeltaSeconds`))) true)
  (set `self.Velocity` (+ (`self.Velocity`) (* (`self.Acceleration`) (`GameplayStatics.GetWorldDeltaSeconds`)))))

(event `Explode`
  (bind (_returnvalue_location _returnvalue_rotation _returnvalue_scale) (`KismetMathLibrary.BreakTransform` (`self.GetTransform`)))
  (`self.K2_DestroyActor`)
  (`GameplayStatics.SpawnEmitterAtLocation` (`self.HitParticle`) _returnvalue_location _returnvalue_rotation _returnvalue_scale))

(event `self.CollisionSphere.OnComponentHit`
  (params (HitComponent :type "PrimitiveComponent Object Reference") (OtherActor :type "Actor Object Reference") (OtherComp :type "PrimitiveComponent Object Reference") (NormalImpulse :type "Vector Structure") (Hit :type "HitResult Structure (by ref)"))
  (if (!= OtherActor (`self.SourceActor`))
    (`self.HitActor` (`self.SourceActor`) OtherActor))
  (`GameplayStatics.PlaySoundAtLocation` (`self.HitSound`) (`self.K2_GetActorLocation`) (struct) 1.0 1.0 0.0 "/Game/DCT/Sound/ATT_Dungeon.ATT_Dungeon" null null :!label _label)
  (`self.Explode`))

(event `self.CollisionSphere.OnComponentBeginOverlap`
  (params (OverlappedComponent :type "PrimitiveComponent Object Reference") (OtherActor :type "Actor Object Reference") (OtherComp :type "PrimitiveComponent Object Reference") (OtherBodyIndex :type Integer) (bFromSweep :type Boolean) (SweepResult :type "HitResult Structure (by ref)"))
  (if (!= OtherActor (`self.SourceActor`))
    (`self.HitActor` (`self.SourceActor`) OtherActor)
    (goto _label)))

(event `HitActor`
  (params (SourceActor :type "Actor Object Reference") (HitActor :type "Actor Object Reference"))
  (bind (_bvalid _effect) (`/Game/DCT/Blueprints/Core/BP_Dungeon_State.GetItemEffectAndSpawnIfNeeded` (`.DungeonState` (`/Game/DCT/Blueprints/Core/BPFL_Singletons.GetDungeonGameState`)) (`self.HeldItem`)))
  (if _bvalid
    (`/Game/DCT/Blueprints/Effects/BP_Effect.ProjectileHit` _effect SourceActor HitActor (`self.HeldItem`))))

(fn `UserConstructionScript`
  (`StaticMeshComponent.SetStaticMesh` (`self.ProjectileMesh`) (`self.Appearance`))
  (`ParticleSystemComponent.SetTemplate` (`self.ProjectileParticle`) (`self.BodyParticle`)))