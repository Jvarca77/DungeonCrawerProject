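; BP_SaveCheckpoint is a dungeon checkpoint actor that saves the game when a BP_DungeonPawn first overlaps it.
; A DoOnce gates the overlap, which applies a small capped Health increase to every player character in the dungeon state, then calls SaveAll on the game instance's DungeonInstance.
; If DisplayText is set, it also shows a WBP_WaveText widget announcing the checkpoint.
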(event `self.ReceiveActorBeginOverlap`
  (params (OtherActor :type "Actor Object Reference"))
  (cast `/Game/DCT/Blueprints/Core/BP_DungeonPawn` OtherActor)
  (`/Engine/EditorBlueprintResources/StandardMacros.DoOnce` false
    (:`Completed`
      (for _array_element (`/Game/DCT/Blueprints/Core/BP_Dungeon_State.PlayerCharacters` (`.DungeonState` (`/Game/DCT/Blueprints/Core/BPFL_Singletons.GetDungeonGameState`)))
        (`/Game/DCT/Blueprints/Core/BP_PlayerCharacter.ModifyStatCapped` _array_element (struct :`TagName` "Stat.Health") 1.0))
      (`/Game/DCT/Blueprints/Core/BP_GI_Dungeon.SaveAll` (`.DungeonInstance` (`/Game/DCT/Blueprints/Core/BPFL_Singletons.GetDungeonGameInstance`)) true)
      (if (`self.bDisplayText`)
        (bind _returnvalue (`|CreateWidget` "/Game/DCT/UserInterface/WBP_WaveText.WBP_WaveText_C" null "CHECKPOINT REACHED"))
        (`UserWidget.AddToViewport` _returnvalue 0)))))

(fn `UserConstructionScript`)