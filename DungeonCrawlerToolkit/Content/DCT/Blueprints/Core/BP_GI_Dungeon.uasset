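; Game instance for the dungeon game that saves and restores characters, held item, settings, player position and per-level state in a BP_CharacterSave slot.
; Saving gathers monsters, items and interactables through BPI_Saveable, stored by level name.
; Loading respawns monsters and items, reconciles interactables by display name, and places the player at the matching transition or saved transform.
; Init also builds a gameplay-tag friendly-name lookup.
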(event `self.ReceiveInit`
  (`self.MakeTagFriendlyNameLookup`)
  (`self.SetupDebugId`))

(event `LoadHeldItem`
  (params (SaveGame :type "/Game/DCT/Blueprints/Core/BP_CharacterSave Object Reference"))
  (bind (_bvalid _dungeonplayercontroller) (`/Game/DCT/Blueprints/Core/BPFL_Singletons.GetDungeonPlayerController`))
  (bind (_helditem_itemtype _helditem_amount) (break `/Game/DCT/Data/FItemSave` (`/Game/DCT/Blueprints/Core/BP_CharacterSave.HeldItem` SaveGame)))
  (bind (_datatable _rowname) (break `DataTableRowHandle` _helditem_itemtype))
  (bind _returnvalue (`DataTableFunctionLibrary.DoesDataTableRowExist` _datatable _rowname))
  (if _returnvalue
    (bind _returnvalue_2 (`|CreateWidget` "/Game/DCT/UserInterface/WBP_Item.WBP_Item_C" _dungeonplayercontroller _helditem_amount _helditem_itemtype))
    (`KismetSystemLibrary.Delay` 0.0)
    (`/Game/DCT/Blueprints/Core/BP_PC_Dungeon.SetMouseWidget` _dungeonplayercontroller _returnvalue_2)))

(fn `ClearStoredActors`
  (`KismetArrayLibrary.Array_Clear` (`self.SavedMonsters`))
  (`KismetArrayLibrary.Array_Clear` (`self.SavedItems`))
  (`KismetArrayLibrary.Array_Clear` (`self.SavedInteractables`))
  (return))

(fn `FindValidTransitionTarget`
  (returns (bValid :type Boolean) (TransitionTarget :type "/Game/DCT/Blueprints/Dungeon/BP_Interact_LevelTransition Object Reference"))
  (bind _outactors (`GameplayStatics.GetAllActorsOfClass` "/Game/DCT/Blueprints/Dungeon/BP_Interact_LevelTransition.BP_Interact_LevelTransition_C"))
  (for _array_element _outactors
    (if (== (`/Game/DCT/Blueprints/Dungeon/BP_Interact_LevelTransition.Identifier` _array_element) (`self.TransitionTarget`))
      (return true _array_element)))
  (return false null))

(fn `GetSavedCharacters`
  (returns (bValid :type Boolean) (PlayerCharacterData :type "Array of /Game/DCT/Data/FCharacterData Structure"))
  (bind _returnvalue (`GameplayStatics.DoesSaveGameExist` (`self.SaveId`)))
  (if _returnvalue
    (bind _returnvalue_2 (`GameplayStatics.LoadGameFromSlot` (`self.SaveId`)))
    (bind _asbp_character_save (cast `/Game/DCT/Blueprints/Core/BP_CharacterSave` _returnvalue_2)
      (:`then`
        (return true (`/Game/DCT/Blueprints/Core/BP_CharacterSave.PlayerCharacterData` _asbp_character_save)))
      (:`CastFailed`
        _)))
  (return false))

(fn `GetSavedGameOrMakeIfInvalid`
  (params (SaveIdIn :type String))
  (returns (SaveGame :type "/Game/DCT/Blueprints/Core/BP_CharacterSave Object Reference"))
  (bind _returnvalue (`GameplayStatics.DoesSaveGameExist` SaveIdIn))
  (if _returnvalue
    (bind _returnvalue_2 (`GameplayStatics.LoadGameFromSlot` SaveIdIn))
    (bind _asbp_character_save (cast `/Game/DCT/Blueprints/Core/BP_CharacterSave` _returnvalue_2))
    (return _asbp_character_save)
    (else
      (bind _returnvalue_3 (`GameplayStatics.CreateSaveGameObject` "/Game/DCT/Blueprints/Core/BP_CharacterSave.BP_CharacterSave_C"))
      (return _returnvalue_3))))

(fn `GetSavedLevel`
  (returns (bValid :type Boolean) (SavedLevel :type String))
  (bind _returnvalue (`GameplayStatics.DoesSaveGameExist` (`self.SaveId`)))
  (if _returnvalue
    (bind _returnvalue_2 (`GameplayStatics.LoadGameFromSlot` (`self.SaveId`)))
    (bind _asbp_character_save (cast `/Game/DCT/Blueprints/Core/BP_CharacterSave` _returnvalue_2)
      (:`then`
        (return true (`/Game/DCT/Blueprints/Core/BP_CharacterSave.SavedLevel` _asbp_character_save)))
      (:`CastFailed`
        (return false "")))
    (else
      (return false ""))))

(fn `Load LevelData`
  (locals (LocalInteractableDisplayNames :type "Array of String") (LocalInteractableIndex :type Integer))
  (bind _returnvalue (`GameplayStatics.DoesSaveGameExist` (`self.SaveId`)))
  (if _returnvalue
    (`self.LoadSettings`)
    (`self.LoadAndSetStartLocation`)
    (bind _returnvalue_2 (`GameplayStatics.LoadGameFromSlot` (`self.SaveId`)))
    (bind _asbp_character_save (cast `/Game/DCT/Blueprints/Core/BP_CharacterSave` _returnvalue_2)
      (:`then`
        (bind _returnvalue_3 (`GameplayStatics.GetCurrentLevelName` true))
        (bind (_value _returnvalue_4) (`BlueprintMapLibrary.Map_Find` (`/Game/DCT/Blueprints/Core/BP_CharacterSave.SavedLevels` _asbp_character_save) _returnvalue_3))
        (if _returnvalue_4
          (bind _outactors (`GameplayStatics.GetAllActorsWithInterface` "/Game/DCT/Blueprints/Core/BPI_Saveable.BPI_Saveable_C"))
          (for _array_element _outactors
            (message `/Game/DCT/Blueprints/Core/BPI_Saveable.UpdatePreplaced` _array_element))
          (`|ExecutionSequence`
            (:`then_0`
              (bind (_monsters _items _interactables) (break `/Game/DCT/Data/FLevelSave` _value))
              (for _array_element_2 _monsters
                (bind (_monsterclass _monstertype _transform _stats) (break `/Game/DCT/Data/FMonsterSave` _array_element_2))
                (`|SpawnActorFromClass` _monsterclass _transform "AlwaysSpawn" "SelectDefaultAtRuntime" null _monstertype _stats null)))
            (:`then_1`
              (`self.UpdateInteractables` _interactables))
            (:`then_2`
              (for _array_element_3 _items
                (bind (_itemtype _amount _transform_2 _benablephysics) (break `/Game/DCT/Data/FItemSave` _array_element_3))
                (`|SpawnActorFromClass` "/Game/DCT/Blueprints/Items/BP_Item.BP_Item_C" _transform_2 "Undefined" "OverrideRootScale" null _amount _itemtype _benablephysics null)))
            (:`then_3`
              (`self.LoadHeldItem` _asbp_character_save))
            (:`then_4`
              (return)))
          (else
            (`self.LoadHeldItem` _asbp_character_save)
            (return))))
      (:`CastFailed`
        (return)))
    (else
      (return))))

(fn `LoadAndSetStartLocation`
  (returns (bFoundValidLocation :type Boolean))
  (bind (_bvalid _transitiontarget) (`self.FindValidTransitionTarget`))
  (if _bvalid
    (bind _returnvalue (`SceneComponent.K2_GetComponentToWorld` (`/Game/DCT/Blueprints/Dungeon/BP_Interact_LevelTransition.ExitArrow` _transitiontarget)))
    (`Actor.K2_SetActorLocationAndRotation` (`GameplayStatics.GetPlayerPawn` 0) (.location _returnvalue) (`KismetMathLibrary.MakeRotator` 0.0 0.0 (.yaw (.rotation _returnvalue))) false false)
    (return true)
    (else
      (switch `name` (`self.TransitionTarget`)
        (:`Default`
          (return false))
        (:`Load`
          (bind _returnvalue_2 (`GameplayStatics.LoadGameFromSlot` (`self.SaveId`)))
          (bind _asbp_character_save (cast `/Game/DCT/Blueprints/Core/BP_CharacterSave` _returnvalue_2)
            (:`then`
              (bind _returnvalue_3 (`GameplayStatics.GetCurrentLevelName` true))
              (bind _savedlevel (`/Game/DCT/Blueprints/Core/BP_CharacterSave.SavedLevel` _asbp_character_save))
              (if (`KismetStringLibrary.EqualEqual_StrStr` _returnvalue_3 _savedlevel)
                (`Actor.K2_SetActorTransform` (`GameplayStatics.GetPlayerPawn` 0) (`/Game/DCT/Blueprints/Core/BP_CharacterSave.PlayerTransform` _asbp_character_save) false false)
                (elif (`KismetTextLibrary.TextIsEmpty` (`KismetTextLibrary.Conv_StringToText` _savedlevel))
                  (return false)
                  (else
                    (`GameplayStatics.OpenLevel` (`KismetStringLibrary.Conv_StringToName` _savedlevel))))))
            (:`CastFailed`
              (return false))))))))

(fn `LoadLastSave`
  (returns (bSuccess :type Boolean))
  (set `self.TransitionTarget` "Load")
  (bind (_bvalid _savedlevel) (`self.GetSavedLevel`))
  (if _bvalid
    (`GameplayStatics.OpenLevel` (`KismetStringLibrary.Conv_StringToName` _savedlevel))
    (return true)
    (else
      (return false))))

(fn `LoadSettings`
  (bind _returnvalue (`GameplayStatics.LoadGameFromSlot` (`self.SaveId`)))
  (bind _asbp_character_save (cast `/Game/DCT/Blueprints/Core/BP_CharacterSave` _returnvalue)
    (:`then`
      (set `self.bInstantMovement` (`/Game/DCT/Blueprints/Core/BP_CharacterSave.bInstantMovement` _asbp_character_save))
      (set `self.bMovementArrows` (`/Game/DCT/Blueprints/Core/BP_CharacterSave.bShowMovementArrows` _asbp_character_save))
      (set `/Game/DCT/Blueprints/Core/BP_DungeonPawn.bInstantMovement` (`self.bInstantMovement`) (`.DungeonPawn` (`/Game/DCT/Blueprints/Core/BPFL_Singletons.GetDungeonPawn`)))
      (return))
    (:`CastFailed`
      (return))))

(fn `MakeTagFriendlyNameLookup`
  (bind _outrownames (`DataTableFunctionLibrary.GetDataTableRowNames` "/Game/DCT/Data/DT_FriendlyTagNames.DT_FriendlyTagNames"))
  (for _array_element _outrownames
    (bind _returnvalue (`|GetDataTableRow` "/Game/DCT/Data/DT_FriendlyTagNames.DT_FriendlyTagNames" _array_element)
      (:`then`
        (bind (_tag _friendlyname) (break `/Game/DCT/Data/FFriendlyTagName` _returnvalue))
        (`BlueprintMapLibrary.Map_Add` (`self.FriendlyTagNames`) _tag _friendlyname))))
  (for _array_element_2 (`BlueprintGameplayTagLibrary.BreakGameplayTagContainer` (`self.StatTags`))
    (if (not (`BlueprintMapLibrary.Map_Contains` (`self.FriendlyTagNames`) _array_element_2))
      (`BlueprintMapLibrary.Map_Add` (`self.FriendlyTagNames`) _array_element_2 (`/Game/DCT/Blueprints/Core/BPFL_Dungeon.GetLowestLevelTagName` _array_element_2))))
  (return))

(fn `SaveAll`
  (params (bSavePawnTransform :type Boolean))
  (if bSavePawnTransform
    (`self.SavePawnTransformAndLevel`))
  (`self.StoreCharacterStats` (`/Game/DCT/Blueprints/Core/BP_Dungeon_State.PlayerCharacters` (`.DungeonState` (`/Game/DCT/Blueprints/Core/BPFL_Singletons.GetDungeonGameState`))) false true)
  (`self.SaveLevel`)
  (`self.SaveSettings`)
  (return))

(fn `SaveLevel`
  (bind _savegame (`self.GetSavedGameOrMakeIfInvalid` (`self.SaveId`)))
  (`self.ClearStoredActors`)
  (bind _outactors (`GameplayStatics.GetAllActorsWithInterface` "/Game/DCT/Blueprints/Core/BPI_Saveable.BPI_Saveable_C"))
  (for _array_element _outactors
    (message `/Game/DCT/Blueprints/Core/BPI_Saveable.SaveActor` _array_element self))
  (bind _returnvalue (`GameplayStatics.GetCurrentLevelName` true))
  (`BlueprintMapLibrary.Map_Add` (`/Game/DCT/Blueprints/Core/BP_CharacterSave.SavedLevels` _savegame) _returnvalue (make `/Game/DCT/Data/FLevelSave` (`self.SavedMonsters`) (`self.SavedItems`) (`self.SavedInteractables`)))
  (`GameplayStatics.SaveGameToSlot` _savegame (`self.SaveId`))
  (return))

(fn `SavePawnTransformAndLevel`
  (bind _savegame (`self.GetSavedGameOrMakeIfInvalid` (`self.SaveId`)))
  (set `/Game/DCT/Blueprints/Core/BP_CharacterSave.PlayerTransform` (`Actor.GetTransform` (`GameplayStatics.GetPlayerPawn` 0)) _savegame)
  (bind _returnvalue (`GameplayStatics.GetCurrentLevelName` true))
  (set `/Game/DCT/Blueprints/Core/BP_CharacterSave.SavedLevel` _returnvalue _savegame)
  (`GameplayStatics.SaveGameToSlot` _savegame (`self.SaveId`))
  (return))

(fn `SaveSettings`
  (bind _savegame (`self.GetSavedGameOrMakeIfInvalid` (`self.SaveId`)))
  (`/Game/DCT/Blueprints/Core/BP_CharacterSave.StoreSettings` _savegame (`self.bInstantMovement`) (`self.bMovementArrows`))
  (`GameplayStatics.SaveGameToSlot` _savegame (`self.SaveId`))
  (return))

(fn `SetRandomSaveId`
  (set `self.SaveId` (`KismetStringLibrary.Conv_DoubleToString` (`KismetMathLibrary.RandomFloat`)))
  (return))

(fn `SetupDebugId`
  (if (`KismetStringLibrary.EqualEqual_StrStr` (`self.SaveId`) "Debug")
    (`self.SetRandomSaveId`)
    (return)
    (else
      (return))))

(fn `StoreCharacterStats`
  (params (PlayerCharacters :type "Array of /Game/DCT/Blueprints/Core/BP_PlayerCharacter Object Reference") (bRebaseCharacters :type Boolean) (bStoreItems :type Boolean))
  (locals (LocalInventory :type "Map of Integer to /Game/DCT/Data/FItemSave Structure") (LocalEquipment :type "Map of Integer to /Game/DCT/Data/FItemSave Structure") (LocalPlayerCharacterData :type "Array of /Game/DCT/Data/FCharacterData Structure") (LocalSaveGame :type "/Game/DCT/Blueprints/Core/BP_CharacterSave Object Reference"))
  (bind (_bvalid _dungeonplayercontroller) (`/Game/DCT/Blueprints/Core/BPFL_Singletons.GetDungeonPlayerController`))
  (bind _mousefollowwidget (`/Game/DCT/Blueprints/Core/BP_PC_Dungeon.MouseFollowWidget` _dungeonplayercontroller))
  (bind _savegame (`self.GetSavedGameOrMakeIfInvalid` (`self.SaveId`)))
  (`/Game/DCT/Blueprints/Core/BP_CharacterSave.StoreCharacters` _savegame (`local.PlayerCharacters`) (`local.bRebaseCharacters`) (`local.bStoreItems`))
  (if _bvalid
    (`/Engine/EditorBlueprintResources/StandardMacros.IsValid` _mousefollowwidget
      (:`Is Valid`
        (set `/Game/DCT/Blueprints/Core/BP_CharacterSave.HeldItem` (make `/Game/DCT/Data/FItemSave` (`/Game/DCT/UserInterface/WBP_Item.ItemType` _mousefollowwidget) (`/Game/DCT/UserInterface/WBP_Item.Amount` _mousefollowwidget) (`KismetMathLibrary.MakeTransform` (0.0 0.0 0.0))) _savegame))
      (:`Is Not Valid`
        (set `/Game/DCT/Blueprints/Core/BP_CharacterSave.HeldItem` (make `/Game/DCT/Data/FItemSave` (struct) 0) _savegame))))
  (`GameplayStatics.SaveGameToSlot` _savegame (`self.SaveId`))
  (return))

(fn `UpdateInteractables`
  (params (LoadedInteractables :type "Array of /Game/DCT/Data/FInteractableSave Structure"))
  (locals (LocalInteractableIndex :type Integer) (LocalInteractableDisplayNames :type "Array of String"))
  (for _array_element LoadedInteractables
    (`KismetArrayLibrary.Array_Add` (`local.LocalInteractableDisplayNames`) (`.DisplayName_17_5E23F766418FD1196F1000913BC2C007` (break `/Game/DCT/Data/FInteractableSave` _array_element))))
  (bind _outactors (`GameplayStatics.GetAllActorsOfClass` "/Game/DCT/Blueprints/Dungeon/BP_Interact.BP_Interact_C"))
  (bind (_arrayindex _arrayelement) (`/Engine/EditorBlueprintResources/StandardMacros.ReverseForEachLoop` _outactors)
    (:`LoopBody`
      (bind _output_get (set `local.LocalInteractableIndex` (`KismetArrayLibrary.Array_Find` (`local.LocalInteractableDisplayNames`) (`KismetSystemLibrary.GetDisplayName` _arrayelement))))
      (if (!= _output_get -1)
        (bind (_displayname _transform _interactstate) (break `/Game/DCT/Data/FInteractableSave` (`|GetArrayItem` (`local.LoadedInteractables`) _output_get)))
        (`Actor.K2_SetActorTransform` _arrayelement _transform false false)
        (`/Game/DCT/Blueprints/Dungeon/BP_Interact.UpdateDesiredState` _arrayelement _interactstate)
        (`KismetArrayLibrary.Array_Remove` (`local.LoadedInteractables`) (`local.LocalInteractableIndex`))
        (`KismetArrayLibrary.Array_Remove` (`local.LocalInteractableDisplayNames`) (`local.LocalInteractableIndex`))
        (else
          (`Actor.K2_DestroyActor` _arrayelement))))
    (:`Completed`
      (for _array_element_2 (`local.LoadedInteractables`)
        (bind (_displayname_2 _transform_2 _interactstate_2 _interactableclass) (break `/Game/DCT/Data/FInteractableSave` _array_element_2))
        (`|SpawnActorFromClass` _interactableclass _transform_2 "AlwaysSpawn" "SelectDefaultAtRuntime" null _interactstate_2 null))
      (return))))