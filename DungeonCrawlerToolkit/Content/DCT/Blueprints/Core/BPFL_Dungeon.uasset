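; Blueprint function library of dungeon helpers for damage stats, gameplay tags and monster alerting.
; GetDamageRange reads min and max damage from a stat map, adds any bonus and truncates, falling back to the bonus alone or zero.
; GetLowestLevelTagName returns a gameplay tag's last dot-separated segment.
; ForceMonstersLookForPlayer makes every BP_Monster look for the first player's pawn on the Visibility channel, alerting if found.
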(fn `ForceMonstersLookForPlayer`
  (bind _outactors (`GameplayStatics.GetAllActorsOfClass` null "/Game/DCT/Blueprints/Monsters/BP_Monster.BP_Monster_C"))
  (for _array_element _outactors
    (`/Game/DCT/Blueprints/Monsters/BP_Monster.LookForActor` _array_element (`GameplayStatics.GetPlayerPawn` null) true "TraceTypeQuery1"))
  (return))

(fn `GetDamageRange`
  (params (Stats :type "Map of GameplayTag Structure to Float (double-precision)"))
  (returns (MinDamage :type Integer) (MaxDamage :type Integer))
  (bind (_value _returnvalue) (`BlueprintMapLibrary.Map_Find` Stats (struct :`TagName` "Stat.MinDamage")))
  (bind (_value_2 _returnvalue_2) (`BlueprintMapLibrary.Map_Find` Stats (struct :`TagName` "Stat.MaxDamage")))
  (bind (_value_3 _returnvalue_3) (`BlueprintMapLibrary.Map_Find` Stats (struct :`TagName` "Stat.DamageBonus")))
  (if (and _returnvalue _returnvalue_2)
    (if _returnvalue_3
      (return (`KismetMathLibrary.FTrunc` (+ _value _value_3)) (`KismetMathLibrary.FTrunc` (+ _value_2 _value_3)))
      (else
        (return (`KismetMathLibrary.FTrunc` _value) (`KismetMathLibrary.FTrunc` _value_2))))
    (elif _returnvalue_3
      (return (`KismetMathLibrary.FTrunc` _value_3) (`KismetMathLibrary.FTrunc` _value_3))
      (else
        (return 0 0)))))

(fn `GetLowestLevelTagName`
  (params (GameplayTag :type "GameplayTag Structure (by ref)"))
  (returns (Name :type String))
  (return (`.RightS` (`KismetStringLibrary.Split` (`KismetStringLibrary.Conv_NameToString` (`BlueprintGameplayTagLibrary.GetTagName` GameplayTag)) "." "IgnoreCase" "FromEnd"))))