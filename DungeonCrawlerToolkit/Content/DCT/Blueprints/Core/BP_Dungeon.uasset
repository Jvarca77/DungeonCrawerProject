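; BP_Dungeon starts up a dungeon level when play begins.
; BeginPlay loads level data through the game instance's dungeon instance, runs the dungeon manager's setup, then fades the camera in from full opacity.
; FadeInCamera issues the hold and fade-out-of-black calls back to back with no delay, so the second immediately replaces the first.
; The character-sheet widget getters are stubs returning index zero and no valid character.
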(event `self.ReceiveBeginPlay`
  (`/Game/DCT/Blueprints/Core/BP_GI_Dungeon.Load LevelData` (`.DungeonInstance` (`/Game/DCT/Blueprints/Core/BPFL_Singletons.GetDungeonGameInstance`)))
  (`/Game/DCT/Blueprints/Core/BP_DungeonManager.Setup` (`.DungeonManager` (`/Game/DCT/Blueprints/Core/BPFL_Singletons.GetDungeonManager`)))
  (`self.FadeInCamera` 0.5))

(fn `FadeInCamera`
  (params (BlackDuration :type "Float (double-precision)" :default 1.0) (FadeDuration :type "Float (double-precision)" :default 1.0))
  (`PlayerCameraManager.StartCameraFade` :`self` (`GameplayStatics.GetPlayerCameraManager` 0) :`FromAlpha` 1.0 :`ToAlpha` 1.0 :`Duration` (`local.BlackDuration`) :`bHoldWhenFinished` true)
  (`PlayerCameraManager.StartCameraFade` :`self` (`GameplayStatics.GetPlayerCameraManager` 0) :`FromAlpha` 1.0 :`Duration` (`local.FadeDuration`) :`bHoldWhenFinished` true)
  (return))

(fn `GetActiveCharacterSheetWidgetIndex`
  (returns (Index :type Integer))
  (return 0))

(fn `GetActiveWidgetCharacter`
  (returns (bValid :type Boolean) (PlayerCharacterRef :type "/Game/DCT/Blueprints/Core/BP_PlayerCharacter Object Reference"))
  (return false null))

(fn `UserConstructionScript`)