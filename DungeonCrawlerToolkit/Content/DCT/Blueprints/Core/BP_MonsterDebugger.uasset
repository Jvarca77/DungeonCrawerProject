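; BP_MonsterDebugger is a debug actor that shows the state of every monster on the dungeon grid.
; Each tick it gathers all BP_Monster actors and converts their grid index to a world position through the dungeon manager.
; It draws a sphere and a label with type, name and health there, turning the text red and marking it DEAD for dead monsters.
; SetEnabledState toggles the overlay by switching actor ticking.
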(event `self.ReceiveBeginPlay`
  (set `self.DungeonManagerRef` (`.DungeonManager` (`/Game/DCT/Blueprints/Core/BPFL_Singletons.GetDungeonManager`)))
  (`self.SetEnabledState` (`self.bEnabled`)))

(event `self.ReceiveTick`
  (params (DeltaSeconds :type "Float (single-precision)"))
  (bind _outactors (`GameplayStatics.GetAllActorsOfClass` "/Game/DCT/Blueprints/Monsters/BP_Monster.BP_Monster_C"))
  (for _array_element _outactors
    (bind _locationout (`/Game/DCT/Blueprints/Core/BP_DungeonManager.ConvertFromGridToWorld` (`self.DungeonManagerRef`) (+ (`BlueprintMapLibrary.Map_Find` (`/Game/DCT/Blueprints/Core/BP_DungeonManager.GridLocations` (`self.DungeonManagerRef`)) (`/Game/DCT/Blueprints/Monsters/BP_Monster.GridIndex` _array_element)) (`self.TextOffset`))))
    (bind (_monstertype_datatable _monstertype_rowname) (break `DataTableRowHandle` (`/Game/DCT/Blueprints/Monsters/BP_Monster.MonsterType` _array_element)))
    (bind _bdead (`/Game/DCT/Blueprints/Monsters/BP_Monster.bDead` _array_element))
    (`KismetSystemLibrary.DrawDebugString` _locationout (`KismetStringLibrary.Concat_StrStr` (`KismetStringLibrary.Conv_NameToString` _monstertype_rowname) " \n" (`KismetSystemLibrary.GetDisplayName` _array_element) " \nHealth: " (`KismetStringLibrary.Conv_DoubleToString` (`BlueprintMapLibrary.Map_Find` (`/Game/DCT/Blueprints/Monsters/BP_Monster.MonsterStats` _array_element) (struct :`TagName` "Stat.Health"))) " \n" (`KismetMathLibrary.SelectString` "DEAD" "" _bdead)) null (`KismetMathLibrary.SelectColor` (struct :`R` 1.0 :`B` 0.004613 :`A` 1.0) (struct :`R` 1.0 :`G` 1.0 :`B` 1.0 :`A` 1.0) _bdead))
    (`KismetSystemLibrary.DrawDebugSphere` _locationout 80.0 6 (struct :`R` 1.0 :`B` 0.75 :`A` 1.0) 0.0 2.0)))

(event `SetEnabledState`
  (params (bEnabled :type Boolean))
  (bind _output_get (set `self.bEnabled` bEnabled))
  (`self.SetActorTickEnabled` _output_get))

(fn `UserConstructionScript`)