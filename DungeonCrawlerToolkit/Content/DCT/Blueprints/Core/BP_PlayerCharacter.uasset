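; Player character object for a dungeon game, holding gameplay-tag-keyed base and current stats built from race and class DataTable rows.
; ModifyStat is the hub: equipment alters current stats, base changes also apply to current, and curve-driven derived stats can cascade.
; Health changes drive damage flash, death and revival; level gains equip class abilities.
; As it cannot tick, regeneration relies on pawn step events and an externally driven tick.
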(event `/Game/DCT/Blueprints/Core/BPI_AttackTarget.TakeDamage`
  (params (Damage :type "Float (double-precision)"))
  (`self.ModifyStat` (`KismetMathLibrary.FMax` (- Damage (`self.GetStatValue` (struct :`TagName` "Stat.Armor")))) (struct :`TagName` "Stat.Health") false "NewEnumerator1"))

(event `BindPawnStepEvent`
  (params (DungeonPawnRef :type "/Game/DCT/Blueprints/Core/BP_DungeonPawn Object Reference"))
  (add `/Game/DCT/Blueprints/Core/BP_DungeonPawn.OnStepEnd` DungeonPawnRef (delegate `EventOnStep`)))

(event `EventOnStep`
  (params (DungeonPawn :type "/Game/DCT/Blueprints/Core/BP_DungeonPawn Object Reference"))
  (if (not (`self.bDead`))
    (`self.ModifyStatCapped` (struct :`TagName` "Stat.Health") (`self.HealthGainOnStep`))))

(fn `AttemptInteract`
  (params (TriggeringActor :type "Actor Object Reference"))
  (returns (bSuccess :type Boolean))
  (return false))

(fn `ChangeCharacterClass`
  (params (NewClass :type "DataTableRowHandle Structure"))
  (bind (_datatable _rowname) (break `DataTableRowHandle` NewClass))
  (bind (_characterclass_datatable _characterclass_rowname) (break `DataTableRowHandle` (`self.CharacterClass`)))
  (`|ExecutionSequence`
    (:`then_0`
      (bind _returnvalue (`|GetDataTableRow` _characterclass_datatable _characterclass_rowname)
        (:`then`
          (`self.ModifyFullStats` (`.Stats_36_3907E16340AE15C1244A959B2CFC6004` (break `/Game/DCT/Data/FStatsMap` _returnvalue)) "NewEnumerator1"))))
    (:`then_1`
      (set `self.CharacterClass` (`local.NewClass`)))
    (:`then_2`
      (bind _returnvalue_2 (`|GetDataTableRow` _datatable _rowname)
        (:`then`
          (`self.ModifyFullStats` (`.Stats_36_3907E16340AE15C1244A959B2CFC6004` (break `/Game/DCT/Data/FStatsMap` _returnvalue_2))))
        (:`RowNotFound`
          _))
      (return))))

(fn `ChangeRace`
  (params (NewRace :type "DataTableRowHandle Structure"))
  (bind (_datatable _rowname) (break `DataTableRowHandle` NewRace))
  (bind (_race_datatable _race_rowname) (break `DataTableRowHandle` (`self.Race`)))
  (`|ExecutionSequence`
    (:`then_0`
      (bind _returnvalue (`|GetDataTableRow` _race_datatable _race_rowname)
        (:`then`
          (`self.ModifyFullStats` (`.Stats_36_3907E16340AE15C1244A959B2CFC6004` (break `/Game/DCT/Data/FStatsMap` _returnvalue)) "NewEnumerator1"))))
    (:`then_1`
      (set `self.Race` (`local.NewRace`)))
    (:`then_2`
      (bind _returnvalue_2 (`|GetDataTableRow` _datatable _rowname)
        (:`then`
          (`self.ModifyFullStats` (`.Stats_36_3907E16340AE15C1244A959B2CFC6004` (break `/Game/DCT/Data/FStatsMap` _returnvalue_2))))
        (:`RowNotFound`
          _))
      (return))))

(fn `CheckIfAllowedInteract`
  (params (TriggeringActor :type "Actor Object Reference"))
  (returns (bAllowed :type Boolean))
  (return false))

(fn `CheckIfEncumbered`
  (returns (bIsEncumbered :type Boolean))
  (return (> (`self.GetStatValue` (struct :`TagName` "Stat.Load")) (`self.GetStatValue` (struct :`TagName` "Stat.MaxLoad")))))

(fn `Equip`
  (params (ItemName :type Name) (bUnequip :type Boolean))
  (locals (LocalItemTables :type "Array of DataTable Object Reference"))
  (for _array_element (`local.LocalItemTables`)
    (bind _returnvalue (`|GetDataTableRow` _array_element ItemName)
      (:`then`
        (`self.ModifyFullStats` (`.EquipStats_151_8B04ED1943498B8F29002D9BD6BA8FF3` (break `/Game/DCT/Data/FItem` _returnvalue)) (select `bool` bUnequip :`false` "NewEnumerator0" :`true` "NewEnumerator1" :!type "/Game/DCT/Data/EManipulate Enum") false)
        (return))))
  (return))

(fn `EquipUnlockedAbilitiesOnLevelUp`
  (params (ChangeInLevels :type "Float (double-precision)"))
  (bind _returnvalue (`KismetMathLibrary.FFloor` ChangeInLevels))
  (bind (_characterclass_datatable _characterclass_rowname) (break `DataTableRowHandle` (`self.CharacterClass`)))
  (if (> _returnvalue 0)
    (`self.OnLevelUp` (`self.GetStatValue` (struct :`TagName` "Stat.Level")))
    (for _index (range _returnvalue)
      (bind _returnvalue_2 (`|GetDataTableRow` _characterclass_datatable _characterclass_rowname)
        (:`then`
          (bind (_value _returnvalue_3) (`BlueprintMapLibrary.Map_Find` (`.AbilityUnlocksByLevel_27_75D29E2B4253D71C40A4C28FD7B85311` (break `/Game/DCT/Data/FStatsMap` _returnvalue_2)) (- (`KismetMathLibrary.FTrunc` (`self.GetStatValue` (struct :`TagName` "Stat.Level"))) _index)))
          (if _returnvalue_3
            (`self.Equip` (`.RowName` (break `DataTableRowHandle` _value)))))
        (:`RowNotFound`
          (return))))
    (return)
    (else
      (return))))

(fn `ExternalTick`
  (params (DeltaSeconds :type "Float (double-precision)"))
  (if (not (`self.bDead`))
    (if (!= (`self.HealthRechargePerSecond`) 0.0)
      (`self.ModifyStatCapped` (struct :`TagName` "Stat.Health") (* DeltaSeconds (`self.HealthRechargePerSecond`))))
    (if (!= (`self.ManaRechargePerSecond`) 0.0)
      (`self.ModifyStatCapped` (struct :`TagName` "Stat.Mana") (* DeltaSeconds (`self.ManaRechargePerSecond`))))
    (return)))

(fn `GetAttachSlot`
  (returns (AttachSlot :type "SceneComponent Object Reference"))
  (return null))

(fn `GetClassName`
  (returns (`Race Tag Row Name` :type Name))
  (bind (_characterclass_datatable _characterclass_rowname) (break `DataTableRowHandle` (`self.CharacterClass`)))
  (return _characterclass_rowname))

(fn `GetDodgeChance`
  (returns (DodgeChance :type "Float (double-precision)"))
  (return 0.0))

(fn `GetItems`
  (returns (InventoryItems :type "Array of /Game/DCT/UserInterface/WBP_Item Object Reference") (EquippedItems :type "Map of /Game/DCT/Data/EItemType Enum to /Game/DCT/UserInterface/WBP_Item Object Reference"))
  (locals (LocalInventoryItems :type "Array of /Game/DCT/UserInterface/WBP_Item Object Reference") (LocalEquippedItems :type "Map of /Game/DCT/Data/EItemType Enum to /Game/DCT/UserInterface/WBP_Item Object Reference"))
  (bind _wbp_inventory (`/Game/DCT/UserInterface/WBP_CharacterSheet.WBP_Inventory` (`self.CharacterSheetRef`)))
  (for _array_element (`PanelWidget.GetAllChildren` (`/Game/DCT/UserInterface/WBP_Inventory.SlotGrid` _wbp_inventory))
    (bind _aswbp_slot (cast `/Game/DCT/UserInterface/WBP_Slot` _array_element))
    (bind _slotteditem (`/Game/DCT/UserInterface/WBP_Slot.SlottedItem` _aswbp_slot))
    (`/Engine/EditorBlueprintResources/StandardMacros.IsValid` _slotteditem
      (:`Is Valid`
        (`KismetArrayLibrary.Array_Add` (`local.LocalInventoryItems`) _slotteditem))))
  (for _array_element_2 (`/Game/DCT/UserInterface/WBP_PaperDoll.Slots` (`/Game/DCT/UserInterface/WBP_Inventory.WBP_PaperDoll` _wbp_inventory))
    (bind _aswbp_slot_2 (cast `/Game/DCT/UserInterface/WBP_Slot` _array_element_2))
    (bind _slotteditem_2 (`/Game/DCT/UserInterface/WBP_Slot.SlottedItem` _aswbp_slot_2))
    (`/Engine/EditorBlueprintResources/StandardMacros.IsValid` _slotteditem_2
      (:`Is Valid`
        (`BlueprintMapLibrary.Map_Add` (`local.LocalEquippedItems`) (`/Game/DCT/UserInterface/WBP_Slot.SlotType` _aswbp_slot_2) _slotteditem_2))))
  (return (`local.LocalInventoryItems`) (`local.LocalEquippedItems`)))

(fn `GetRaceName`
  (returns (`Race Tag Row Name` :type Name))
  (bind (_race_datatable _race_rowname) (break `DataTableRowHandle` (`self.Race`)))
  (return _race_rowname))

(fn `GetStatModifier`
  (params (Stat :type "GameplayTag Structure"))
  (returns (StatMoification :type "Float (double-precision)"))
  (return (- (`BlueprintMapLibrary.Map_Find` (`self.CurrentStats`) Stat) (`BlueprintMapLibrary.Map_Find` (`self.BaseStats`) Stat))))

(fn `GetStatValue`
  (params (Stat :type "GameplayTag Structure") (bBaseStat :type Boolean))
  (returns (StatValue :type "Float (double-precision)"))
  (if bBaseStat
    (return (`BlueprintMapLibrary.Map_Find` (`self.BaseStats`) Stat))
    (else
      (return (`BlueprintMapLibrary.Map_Find` (`self.CurrentStats`) Stat)))))

(fn `KillPlayerCharacter`
  (set `self.bDead` true)
  (`self.OnKilled` self)
  (return))

(fn `ModifyFullStats`
  (params (SourceStats :type "Map of GameplayTag Structure to Float (double-precision) (by ref)") (Manipulation :type "/Game/DCT/Data/EManipulate Enum" :default "NewEnumerator0") (bChangeBaseStat :type Boolean :default true) (bUpdateDerivedStats :type Boolean :default true))
  (bind _keys (`BlueprintMapLibrary.Map_Keys` SourceStats))
  (for _array_element _keys
    (`self.ModifyStat` (`BlueprintMapLibrary.Map_Find` (`local.SourceStats`) _array_element) _array_element bChangeBaseStat (`local.Manipulation`) bUpdateDerivedStats true))
  (return))

(fn `ModifyStat`
  (params (Modifier :type "Float (double-precision)") (Stat :type "GameplayTag Structure") (bChangeBaseStat :type Boolean) (Manipulation :type "/Game/DCT/Data/EManipulate Enum" :default "NewEnumerator0") (bUpdateDerivedStats :type Boolean :default true) (bCanBeNegative :type Boolean))
  (returns (bSuccess :type Boolean) (NewValue :type "Float (double-precision)"))
  (locals (LocalStats :type "Map of GameplayTag Structure to Float (double-precision)") (StatValuePreModification :type "Float (double-precision)"))
  (bind _modifier (`local.Modifier`))
  (bind _localstats (`local.LocalStats`))
  (bind (_value _returnvalue) (`BlueprintMapLibrary.Map_Find` (`local.LocalStats`) (`local.Stat`)))
  (bind _returnvalue_2 (select `/Game/DCT/Data/EManipulate` (`local.Manipulation`) :`NewEnumerator0` (+ _value _modifier) :`NewEnumerator1` (- _value _modifier) :`NewEnumerator2` _modifier))
  (if bChangeBaseStat
    (set `local.LocalStats` (`self.BaseStats`))
    (else
      (set `local.LocalStats` (`self.CurrentStats`))))
  (if _returnvalue
    (set `local.StatValuePreModification` _value)
    (`BlueprintMapLibrary.Map_Add` (`local.LocalStats`) (`local.Stat`) (`KismetMathLibrary.SelectFloat` _returnvalue_2 (`KismetMathLibrary.FMax` _returnvalue_2) (`local.bCanBeNegative`)))
    (if (`local.bChangeBaseStat`)
      (set `self.BaseStats` _localstats)
      (else
        (set `self.CurrentStats` _localstats)))
    (if (`local.bChangeBaseStat`)
      (`self.ModifyStat` (`local.Modifier`) (`local.Stat`) false (`local.Manipulation`) true (`local.bCanBeNegative`))
      (elif (`local.bUpdateDerivedStats`)
        (`self.UpdateDerivedStats` (`local.Stat`) (`local.StatValuePreModification`) (`BlueprintMapLibrary.Map_Find` (`local.LocalStats`) (`local.Stat`)))))
    (`self.RunEffectsFollowingStatChange` (`local.Stat`) (- (`BlueprintMapLibrary.Map_Find` (`local.LocalStats`) (`local.Stat`)) (`local.StatValuePreModification`)) (`local.bChangeBaseStat`))
    (return true (`BlueprintMapLibrary.Map_Find` (`local.LocalStats`) (`local.Stat`)))
    (else
      (return false 0.0))))

(fn `ModifyStatCapped`
  (params (Stat :type "GameplayTag Structure") (Amount :type "Float (double-precision)"))
  (bind _statvalue (`self.GetStatValue` Stat true))
  (bind _statvalue_2 (`self.GetStatValue` Stat))
  (if (< _statvalue_2 _statvalue)
    (`self.ModifyStat` (`KismetMathLibrary.FMin` (+ Amount _statvalue_2) (`KismetMathLibrary.FMax` _statvalue_2 _statvalue)) (`local.Stat`) false "NewEnumerator2")
    (return)
    (else
      (return))))

(fn `ResolveDamageAndDeathEffects`
  (params (HealthChange :type "Float (double-precision)"))
  (bind _minicharacterref (`self.MiniCharacterRef`))
  (if (`self.bDead`)
    (if (> (`self.GetStatValue` (struct :`TagName` "Stat.Health")) 0.0)
      (`self.RevivePlayerCharacter`)
      (return)
      (else
        (return)))
    (else
      (`|ExecutionSequence`
        (:`then_0`
          (if (< (`local.HealthChange`) 0.0)
            (`/Engine/EditorBlueprintResources/StandardMacros.IsValid` _minicharacterref
              (:`Is Valid`
                (`/Game/DCT/UserInterface/WBP_MiniCharacter.RunDamageFlash` _minicharacterref)
                (return))
              (:`Is Not Valid`
                (return)))))
        (:`then_1`
          (if (< (`self.GetStatValue` (struct :`TagName` "Stat.Health")) 1.0)
            (`self.KillPlayerCharacter`)
            (return)
            (else
              (return))))))))

(fn `RevivePlayerCharacter`
  (set `self.bDead` false)
  (`self.OnRevived` self)
  (return))

(fn `RunEffectsFollowingStatChange`
  (params (Stat :type "GameplayTag Structure") (StatChange :type "Float (double-precision)") (bBaseStat :type Boolean))
  (if bBaseStat
    (return)
    (else
      (`|SwitchGameplayTag` Stat
        (:`Default`
          (return))
        (:`Stat.Health`
          (`self.ResolveDamageAndDeathEffects` (`local.StatChange`))
          (return))
        (:`Stat.Level`
          (`self.EquipUnlockedAbilitiesOnLevelUp` (`local.StatChange`))
          (return))))))

(fn `SetupStats`
  (params (StatToUse :type "GameplayTagContainer Structure (by ref)"))
  (bind (_race_datatable _race_rowname) (break `DataTableRowHandle` (`self.Race`)))
  (bind (_characterclass_datatable _characterclass_rowname) (break `DataTableRowHandle` (`self.CharacterClass`)))
  (for _array_element (`BlueprintGameplayTagLibrary.BreakGameplayTagContainer` StatToUse)
    (`BlueprintMapLibrary.Map_Add` (`self.BaseStats`) _array_element))
  (set `self.CurrentStats` (`self.BaseStats`))
  (bind _returnvalue (`|GetDataTableRow` _race_datatable _race_rowname)
    (:`then`
      (`self.ModifyFullStats` (`.Stats_36_3907E16340AE15C1244A959B2CFC6004` (break `/Game/DCT/Data/FStatsMap` _returnvalue))))
    (:`RowNotFound`
      _))
  (bind _returnvalue_2 (`|GetDataTableRow` _characterclass_datatable _characterclass_rowname)
    (:`then`
      (`self.ModifyFullStats` (`.Stats_36_3907E16340AE15C1244A959B2CFC6004` (break `/Game/DCT/Data/FStatsMap` _returnvalue_2)))
      (return))
    (:`RowNotFound`
      (return))))

(fn `UpdateDerivedStats`
  (params (Stat :type "GameplayTag Structure") (StatValuePreModification :type "Float (double-precision)") (CurrentStatValue :type "Float (double-precision)"))
  (bind (_bvalid _statdata) (`self.GetStatDataFromTable` "/Game/DCT/Data/DT_DerivedStats.DT_DerivedStats" "Stat" (`local.Stat`)))
  (if _bvalid
    (for _array_element (`.DerivedStats_6_2DB2EDC64BF541759EDD979C788597BB` (break `/Game/DCT/Data/FStatCurves` _statdata))
      (bind (_derivedstatstat _curve _multiplier) (break `/Game/DCT/Data/FDerivedStatCurve` _array_element))
      (bind _returnvalue (* (- (`CurveFloat.GetFloatValue` _curve (`local.CurrentStatValue`)) (`CurveFloat.GetFloatValue` _curve (`local.StatValuePreModification`))) _multiplier))
      (if (!= _returnvalue 0.0)
        (`self.ModifyStat` _returnvalue _derivedstatstat true "NewEnumerator0" false true)))
    (return)
    (else
      (return))))