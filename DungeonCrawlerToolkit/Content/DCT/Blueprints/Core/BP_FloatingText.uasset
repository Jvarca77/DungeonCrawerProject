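; Floating text actor that shows a string in the world, drifts upward and destroys itself after a short lifetime.
; On BeginPlay, two SmoothLerp nodes run from one sequence: a quick one grows the text size, while a longer reversed one fades alpha.
; The longer lerp also raises the text and turns the actor toward the player camera each update.
; SetColor sets the text's render color.
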(event `self.ReceiveBeginPlay`
  (bind (_textrendercolor_b _textrendercolor_g _textrendercolor_r) (break `Color` (`TextRenderComponent.TextRenderColor` (`self.TextRender`))))
  (`TextRenderComponent.K2_SetText` (`self.TextRender`) (`self.TextToDisplay`))
  (`|ExecutionSequence`
    (:`then_0`
      (bind _alpha (`/Game/DCT/Blueprints/Core/BPML_Utility.SmoothLerp` 2.0 "/Game/DCT/Data/Curve_Smooth_Float.Curve_Smooth_Float" 1.0 true)
        (:`Update`
          (`TextRenderComponent.SetTextRenderColor` (`self.TextRender`) (make `Color` _textrendercolor_b _textrendercolor_g _textrendercolor_r (`KismetMathLibrary.Conv_IntToByte` (`KismetMathLibrary.FFloor` (* (`self.TextStartAlpha`) _alpha)))))
          (`SceneComponent.K2_AddLocalOffset` (`self.TextRender`) (0.0 0.0 0.2) false false)
          (`self.K2_SetActorRotation` (`KismetMathLibrary.FindLookAtRotation` (`self.K2_GetActorLocation`) (`PlayerCameraManager.GetCameraLocation` (`GameplayStatics.GetPlayerCameraManager` 0)))))
        (:`Finished`
          (`self.K2_DestroyActor`))))
    (:`then_1`
      (bind _alpha_2 (`/Game/DCT/Blueprints/Core/BPML_Utility.SmoothLerp` 0.4 "/Game/DCT/Data/Curve_Normal_Float.Curve_Normal_Float")
        (:`Update`
          (`TextRenderComponent.SetWorldSize` (`self.TextRender`) (+ (* _alpha_2 6.0) 26.0)))))))

(fn `SetColor`
  (params (Color :type "LinearColor Structure"))
  (`TextRenderComponent.SetTextRenderColor` (`self.TextRender`) (`KismetMathLibrary.Conv_LinearColorToColor` Color))
  (return))

(fn `UserConstructionScript`)