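; Player pawn for a grid-based dungeon crawler, carrying the party's camera and relaying ticks and damage to every character in game state.
; Input drives tile steps and 90-degree turns, tweened or instant, validated through DungeonManager with wall bumps and encumbrance blocking.
; Completed steps alert nearby monsters, and pathfinding maps are cached per grid index.
; Held mouse look snaps facing past 45 degrees, and Peak/Unpeak blends the camera to targets.
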(event `self.ReceiveBeginPlay`
  ;[0 0 0] Begin Play
  (`KismetSystemLibrary.Delay` 0.1)
  (bind (_gridindex _tilelocation) (`/Game/DCT/Blueprints/Core/BP_DungeonManager.FindNearbyValidTile` (`self.DungeonManagerRef`) (`self.K2_GetActorLocation`)))
  (set `self.GridIndex` _gridindex)
  (`self.K2_SetActorLocation` _tilelocation)
  (for _array_element (`/Game/DCT/Blueprints/Core/BP_Dungeon_State.PlayerCharacters` (`.DungeonState` (`/Game/DCT/Blueprints/Core/BPFL_Singletons.GetDungeonGameState`)))
    (`/Game/DCT/Blueprints/Core/BP_PlayerCharacter.BindPawnStepEvent` _array_element self))
  (set `self.bAllowMovement` true))

(event `Step`
  (params (TargetLocation :type "Vector Structure"))
  ;[0 0 0] Move Step
  (bind ___ (`/Game/DCT/Blueprints/Core/BPML_Utility.MakeLocalVariable` (`self.K2_GetActorLocation`)))
  (`self.UpdateGridIndex` TargetLocation)
  (`|ExecutionSequence`
    (:`then_0`
      (`GameplayStatics.PlaySoundAtLocation` "/Game/DCT/Sound/MSS_Step.MSS_Step" (`self.K2_GetActorLocation`) (struct) 1.5 1.0 0.0 null null null null)
      (set `self.FootstepTracker` (mod (+ (`self.FootstepTracker`) (`KismetMathLibrary.RandomIntegerInRange` 1 3)) 4))
      (if (`self.bInstantMovement`)
        (`self.K2_SetActorLocation` TargetLocation)
        (set `self.bAllowMovement` true :!label _label)
        (`self.OnStepEnd` self)
        (`self.AlertNearbyMonsters`)
        (else
          (bind _alpha (`/Game/DCT/Blueprints/Core/BPML_Utility.SmoothLerp` (`self.MoveSpeedSeconds`) "/Game/DCT/Data/Curve_Linear_Float.Curve_Linear_Float" 1.5)
            (:`Update`
              (`self.K2_SetActorLocation` (`KismetMathLibrary.VLerp` ___ TargetLocation _alpha)))
            (:`Finished`
              (goto _label))))))
    (:`then_1`
      (if (not (`self.bInstantMovement`))
        (bind _alpha_2 (`/Game/DCT/Blueprints/Core/BPML_Utility.SmoothLerp` 0.6 "/Game/DCT/Data/Curve_Normal_Float.Curve_Normal_Float" 1.5)
          (:`Update`
            (`SceneComponent.K2_SetRelativeLocation` (`self.Camera`) (`KismetMathLibrary.MakeVector` 0.0 0.0 (* _alpha_2 5.0)) false false)))))))

(event `EnhancedInput|/Game/DCT/Input/IA_Step`
  (params (ActionValue :type "Vector2D Structure") (ElapsedSeconds :type "Float (double-precision)") (TriggeredSeconds :type "Float (double-precision)") (InputAction :type "InputAction Object Reference" :default "/Game/DCT/Input/IA_Step.IA_Step"))
  (bind (_x _y) (`KismetMathLibrary.BreakVector2D` ActionValue))
  ;[0 0 0] Move Input
  (:`Triggered`
    (if (not (`self.bInstantMovement`))
      (if (!= _x 0.0) :!label _label_2
        (set `self.CurrentMoveDirection` (select `bool` (> _x 0.0) :`false` "NewEnumerator3" :`true` "NewEnumerator2" :!type "/Game/DCT/Data/ERelativeDirection Enum"))
        (else
          (set `self.CurrentMoveDirection` (select `bool` (> _y 0.0) :`false` "NewEnumerator1" :`true` "NewEnumerator0" :!type "/Game/DCT/Data/ERelativeDirection Enum"))))
      (`/Engine/EditorBlueprintResources/StandardMacros.IsValid` (`self.CurrentPeakTarget`)
        (:`Is Valid`
          (`self.Unpeak`))
        (:`Is Not Valid`
          (if (`self.bAllowMovement`)
            (set `self.bAllowMovement` false)
            (`self.AttemptMoveInDirection` (`self.CurrentMoveDirection`)))))))
  (:`Started`
    (if (`self.bInstantMovement`)
      (goto _label_2))))

(event `WallBump`
  (params (Direction :type "/Game/DCT/Data/ERelativeDirection Enum" :default "NewEnumerator0"))
  ;[0 0 0] Wall Bump
  (if (`self.bInstantMovement`)
    (set `self.bAllowMovement` true)
    (else
      (bind ___ (`/Game/DCT/Blueprints/Core/BPML_Utility.MakeLocalVariable` (`self.K2_GetActorLocation`)))
      (bind ____2 (`/Game/DCT/Blueprints/Core/BPML_Utility.MakeLocalVariable` (+ (`self.K2_GetActorLocation`) (* (`/Game/DCT/Blueprints/Core/BP_DungeonManager.GetActorDirectionVector` (`self.DungeonManagerRef`) Direction self) 200.0))))
      (bind _alpha (`/Game/DCT/Blueprints/Core/BPML_Utility.SmoothLerp` 0.4 "/Game/DCT/Data/Curve_Bump_Float.Curve_Bump_Float" 1.5)
        (:`Update`
          (`self.K2_SetActorLocation` (`KismetMathLibrary.VLerp` ___ ____2 (* _alpha 0.1))))
        (:`Finished`
          (set `self.bAllowMovement` true))))))

(event `EnhancedInput|/Game/DCT/Input/IA_Turn`
  (params (ActionValue :type "Float (double-precision)") (ElapsedSeconds :type "Float (double-precision)") (TriggeredSeconds :type "Float (double-precision)") (InputAction :type "InputAction Object Reference" :default "/Game/DCT/Input/IA_Turn.IA_Turn"))
  (bind _returnvalue (`KismetMathLibrary.SignOfFloat` ActionValue))
  (bind _returnvalue_2 (`self.K2_GetActorRotation`))
  (bind _returnvalue_3 (`KismetMathLibrary.ComposeRotators` _returnvalue_2 (`KismetMathLibrary.MakeRotator` 0.0 0.0 (* _returnvalue 90.0))))
  ;[0 0 0] Move Turn
  (:`Triggered`
    (if (not (`self.bInstantMovement`))
      (if (!= _returnvalue 0.0) :!label _label_3
        (if (not (`self.bMouseLookActive`))
          (set `self.bReturnFromMouseLook` false)
          (`/Engine/EditorBlueprintResources/StandardMacros.IsValid` (`self.CurrentPeakTarget`)
            (:`Is Not Valid`
              (if (`self.bInstantMovement`)
                (`self.K2_SetActorRotation` _returnvalue_3)
                (else
                  (`/Engine/EditorBlueprintResources/StandardMacros.DoOnce` false :!label _label_4
                    (:`Completed`
                      (bind ___ (`/Game/DCT/Blueprints/Core/BPML_Utility.MakeLocalVariable` _returnvalue_2))
                      (bind ____2 (`/Game/DCT/Blueprints/Core/BPML_Utility.MakeLocalVariable` _returnvalue_3))
                      (bind _alpha (`/Game/DCT/Blueprints/Core/BPML_Utility.SmoothLerp` (`self.TurnTimeSeconds`) "/Game/DCT/Data/Curve_Smooth_Float.Curve_Smooth_Float" 1.5)
                        (:`Update`
                          (`self.K2_SetActorRotation` (`KismetMathLibrary.RLerp` ___ ____2 _alpha true)))
                        (:`Finished`
                          (goto _label_4 :!via `Reset`)))))))))))))
  (:`Started`
    (if (`self.bInstantMovement`)
      (goto _label_3))))

(event `NotifyEncumbered`
  (params (EncumberedCharacter :type "/Game/DCT/Blueprints/Core/BP_PlayerCharacter Object Reference"))
  ;[0 0 0] Encumberance
  (`/Engine/EditorBlueprintResources/StandardMacros.DoOnce` false :!label _label_5
    (:`Completed`
      (message `/Game/DCT/Blueprints/Core/BPI_PlayerController.DisplayWarning` (`GameplayStatics.GetPlayerController` 0) (`KismetTextLibrary.Conv_StringToText` (`KismetStringLibrary.Concat_StrStr` "You cannot move while " (`KismetStringLibrary.Conv_NameToString` (`/Game/DCT/Blueprints/Core/BP_PlayerCharacter.Name` EncumberedCharacter)) " is encumbered")))
      (`KismetSystemLibrary.Delay` 0.5)
      (set `self.bAllowMovement` true)
      (goto _label_5 :!via `Reset`))))

(event `Peak`
  (params (PeakTransform :type "Transform Structure") (PeakTarget :type "Actor Object Reference"))
  ;[0 0 0] Peak
  (`/Engine/EditorBlueprintResources/StandardMacros.IsValid` (`self.CurrentPeakTarget`)
    (:`Is Not Valid`
      (`/Game/DCT/Blueprints/Core/BPML_Utility.DelayWhile` (not (`self.bAllowMovement`))
        (:`Continue`
          (set `self.CurrentPeakTarget` PeakTarget)
          (bind ___ (`/Game/DCT/Blueprints/Core/BPML_Utility.MakeLocalVariable` (`SceneComponent.K2_GetComponentToWorld` (`self.Camera`))))
          (`self.DisableInput` (`GameplayStatics.GetPlayerController` 0))
          (bind _alpha (`/Game/DCT/Blueprints/Core/BPML_Utility.SmoothLerp` 1.0 "/Game/DCT/Data/Curve_Smooth_Float.Curve_Smooth_Float")
            (:`Update`
              (`SceneComponent.K2_SetWorldTransform` (`self.Camera`) (`KismetMathLibrary.TLerp` ___ PeakTransform _alpha) false false))
            (:`Finished`
              (`self.EnableInput` (`GameplayStatics.GetPlayerController` 0)))))))))

(event `self.ReceiveTick`
  (params (DeltaSeconds :type "Float (single-precision)"))
  ;[0 0 0] Tick
  (for _array_element (`/Game/DCT/Blueprints/Core/BP_Dungeon_State.PlayerCharacters` (`.DungeonState` (`/Game/DCT/Blueprints/Core/BPFL_Singletons.GetDungeonGameState`)))
    (`/Game/DCT/Blueprints/Core/BP_PlayerCharacter.ExternalTick` _array_element DeltaSeconds))
  (`/Engine/EditorBlueprintResources/StandardMacros.Gate` false :!label _label_6
    (:`Exit`
      (`Controller.SetControlRotation` (`GameplayStatics.GetPlayerController` 0) (`KismetMathLibrary.RInterpTo` (`Controller.GetControlRotation` (`GameplayStatics.GetPlayerController` 0)) (`self.K2_GetActorRotation`) (`GameplayStatics.GetWorldDeltaSeconds`) (`KismetMathLibrary.SelectFloat` (`self.MouseLookInterpSpeed`) (`self.TurnInterpSpeed`) (`self.bReturnFromMouseLook`)))))))

(event `EnhancedInput|/Game/DCT/Input/IA_MouseLook`
  (params (ActionValue :type "Vector2D Structure") (ElapsedSeconds :type "Float (double-precision)") (TriggeredSeconds :type "Float (double-precision)") (InputAction :type "InputAction Object Reference" :default "/Game/DCT/Input/IA_MouseLook.IA_MouseLook"))
  (bind (_x _y) (`KismetMathLibrary.BreakVector2D` ActionValue))
  (bind (_returnvalue_roll _returnvalue_pitch _returnvalue_yaw) (`KismetMathLibrary.BreakRotator` (`self.K2_GetActorRotation`)))
  (bind (_returnvalue_roll_2 _returnvalue_pitch_2 _returnvalue_yaw_2) (`KismetMathLibrary.BreakRotator` (`KismetMathLibrary.NormalizedDeltaRotator` (`self.GetControlRotation`) (`self.K2_GetActorRotation`))))
  ;[0 0 0] Mouse Look
  (:`Triggered`
    (if (`self.bMouseLookActive`)
      (`self.AddControllerPitchInput` _y)
      (`self.AddControllerYawInput` _x)
      (if (!= _x 0.0)
        (if (> (`KismetMathLibrary.Abs` _returnvalue_yaw_2) 45.0)
          (`self.K2_SetActorRotation` (`KismetMathLibrary.MakeRotator` _returnvalue_roll _returnvalue_pitch (+ _returnvalue_yaw (* (`KismetMathLibrary.SignOfFloat` _returnvalue_yaw_2) 90.0)))))))))

(event `EnhancedInput|/Game/DCT/Input/IA_TriggerMouseLook`
  (params (ActionValue :type Boolean) (ElapsedSeconds :type "Float (double-precision)") (TriggeredSeconds :type "Float (double-precision)") (InputAction :type "InputAction Object Reference" :default "/Game/DCT/Input/IA_TriggerMouseLook.IA_TriggerMouseLook"))
  ;[0 0 0] Tick
  (:`Started`
    (set `self.bMouseLookActive` true)
    (goto _label_6 :!via `Close`))
  (:`Canceled`
    (set `self.bMouseLookActive` false :!label _label_7)
    (set `self.bReturnFromMouseLook` true)
    (goto _label_6 :!via `Open`))
  (:`Completed`
    (goto _label_7)))

(event `Unpeak`
  ;[0 0 0] Peak
  (`self.DisableInput` (`GameplayStatics.GetPlayerController` 0))
  (bind ___ (`/Game/DCT/Blueprints/Core/BPML_Utility.MakeLocalVariable` (`SceneComponent.GetRelativeTransform` (`self.Camera`))))
  (bind _alpha (`/Game/DCT/Blueprints/Core/BPML_Utility.SmoothLerp` 1.0 "/Game/DCT/Data/Curve_Smooth_Float.Curve_Smooth_Float")
    (:`Update`
      (`SceneComponent.K2_SetRelativeTransform` (`self.Camera`) (`KismetMathLibrary.TLerp` ___ (`KismetMathLibrary.MakeTransform` (0.0 0.0 0.0)) _alpha) false false))
    (:`Finished`
      (set `self.CurrentPeakTarget` null)
      (`self.EnableInput` (`GameplayStatics.GetPlayerController` 0)))))

(event `/Game/DCT/Blueprints/Core/BPI_AttackTarget.TakeDamage`
  (params (Damage :type "Float (double-precision)"))
  ;[0 0 0] Take Damage
  (for _array_element (`/Game/DCT/Blueprints/Core/BP_Dungeon_State.PlayerCharacters` (`.DungeonState` (`/Game/DCT/Blueprints/Core/BPFL_Singletons.GetDungeonGameState`)))
    (message `/Game/DCT/Blueprints/Core/BPI_AttackTarget.TakeDamage` _array_element Damage)))

(event `AlertNearbyMonsters`
  ;[0 0 0] Alert Monsters
  (bind _outactors (`GameplayStatics.GetAllActorsOfClass` "/Game/DCT/Blueprints/Monsters/BP_Monster.BP_Monster_C"))
  (for _array_element _outactors
    (`/Game/DCT/Blueprints/Monsters/BP_Monster.LookForActor` _array_element self true "TraceTypeQuery1")))

(event `EnhancedInput|/Game/DCT/Input/IA_Interact`
  (params (ActionValue :type Boolean) (ElapsedSeconds :type "Float (double-precision)") (TriggeredSeconds :type "Float (double-precision)") (InputAction :type "InputAction Object Reference" :default "/Game/DCT/Input/IA_Interact.IA_Interact"))
  ;[0 0 0] Click interact
  (:`Started`
    (bind _asbp_pc_dungeon (cast `/Game/DCT/Blueprints/Core/BP_PC_Dungeon` (`GameplayStatics.GetPlayerController` 0)))
    (`/Game/DCT/Blueprints/Core/BP_PC_Dungeon.ScreenInteract` _asbp_pc_dungeon)))

(fn `AttemptInteract`
  (params (TriggeringActor :type "Actor Object Reference"))
  (returns (bSuccess :type Boolean))
  (return false))

(fn `AttemptMoveInDirection`
  (params (Direction :type "/Game/DCT/Data/ERelativeDirection Enum" :default "NewEnumerator0"))
  (bind (_bfoundvalidtile _btileisunoccupied _adjacenttilelocation) (`/Game/DCT/Blueprints/Core/BP_DungeonManager.GetAdjacentTileFromLocation` (`self.DungeonManagerRef`) self Direction))
  (if _bfoundvalidtile
    (`/Game/DCT/Blueprints/Core/BPML_Utility.MakeLocalVariable` (`self.K2_GetActorLocation`))
    (if _btileisunoccupied
      (bind (_bisencumbered _encumberedcharacter) (`self.CheckIfEncumbered`))
      (if _bisencumbered
        (`self.NotifyEncumbered` _encumberedcharacter)
        (return)
        (else
          (`self.Step` _adjacenttilelocation)
          (return)))
      (else
        _)))
  (`self.WallBump` Direction)
  (return))

(fn `CheckIfAllowedInteract`
  (params (TriggeringActor :type "Actor Object Reference"))
  (returns (bAllowed :type Boolean))
  (return false))

(fn `CheckIfEncumbered`
  (returns (bIsEncumbered :type Boolean) (EncumberedCharacter :type "/Game/DCT/Blueprints/Core/BP_PlayerCharacter Object Reference"))
  (for _array_element (`/Game/DCT/Blueprints/Core/BP_Dungeon_State.PlayerCharacters` (`.DungeonState` (`/Game/DCT/Blueprints/Core/BPFL_Singletons.GetDungeonGameState`)))
    (bind _bisencumbered (`/Game/DCT/Blueprints/Core/BP_PlayerCharacter.CheckIfEncumbered` _array_element))
    (if _bisencumbered
      (return true _array_element)))
  (return false null))

(fn `GetAttachSlot`
  (returns (AttachSlot :type "SceneComponent Object Reference"))
  (return null))

(fn `GetDodgeChance`
  (returns (DodgeChance :type "Float (double-precision)"))
  (return 0.0))

(fn `GetGridIndex`
  (returns (GridIndex :type Integer))
  (return (`self.GridIndex`)))

(fn `GetWeight`
  (returns (Weight :type "Float (double-precision)"))
  (return (`self.Weight`)))

(fn `MakeStoredPathMapInvalid`
  (set `self.LastStoredPathIndex` -1)
  (return))

(fn `RequestPathMap`
  (returns (StoredPaths :type "Map of Integer to /Game/DCT/Data/FPathfindingMap Structure"))
  (if (not (and (== (`self.GridIndex`) (`self.LastStoredPathIndex`)) (> (`BlueprintMapLibrary.Map_Length` (`self.StoredPaths`)) 0)))
    (set `self.LastStoredPathIndex` (`self.GridIndex`))
    (bind _pathsmap (`/Game/DCT/Blueprints/Core/BP_DungeonManager.RunPathfinding` (`self.DungeonManagerRef`) (`self.GridIndex`) (`self.PathfindingRange`) -1 true))
    (bind _output_get (set `self.StoredPaths` _pathsmap))
    (`/Game/DCT/Blueprints/Core/BP_DungeonManager.DebugDisplayPathfinding` (`self.DungeonManagerRef`) _output_get))
  (return (`self.StoredPaths`)))

(fn `UpdateGridIndex`
  (params (Location :type "Vector Structure"))
  (set `self.GridIndex` (`/Game/DCT/Blueprints/Core/BP_DungeonManager.ConvertLocationToIndex` (`self.DungeonManagerRef`) Location))
  (return))

(fn `UserConstructionScript`
  (bind _returnvalue (`GameplayStatics.GetActorOfClass` "/Game/DCT/Blueprints/Core/BP_DungeonManager.BP_DungeonManager_C"))
  (set `self.DungeonManagerRef` _returnvalue))