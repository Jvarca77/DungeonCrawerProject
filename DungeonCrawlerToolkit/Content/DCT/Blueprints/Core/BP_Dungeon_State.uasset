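; Dungeon state Blueprint that manages the player party, item rules and active character sheet.
; BeginPlay builds characters from the save or default DataTable, triggers UI setup and loads starting items.
; When the last character dies, it shows game over, fades out and reopens the saved level.
; Item use, slotting and pickup run through DataTable-referenced effect actors and rule objects, lazily created and cached per class.
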(event `self.ReceiveBeginPlay`
  (bind (_bvalid _dungeonplayercontroller) (`/Game/DCT/Blueprints/Core/BPFL_Singletons.GetDungeonPlayerController`))
  (bind (_bvalid_2 _dungeoninstance) (`/Game/DCT/Blueprints/Core/BPFL_Singletons.GetDungeonGameInstance`))
  ;[0 0 0] Begin Play
  (if _bvalid_2
    (bind (_bvalid_3 _playercharacterdata) (`/Game/DCT/Blueprints/Core/BP_GI_Dungeon.GetSavedCharacters` _dungeoninstance))
    (if _bvalid_3
      (bind _playercharacters (`self.ConstructStoredPlayerCharacters` _playercharacterdata))
      (set `self.PlayerCharacters` _playercharacters)
      (else
        (bind _playercharacters_2 (`self.ConstructAndSetupDefaultPlayerCharacters`))
        (set `self.PlayerCharacters` _playercharacters_2)
        (set `/Game/DCT/Blueprints/Core/BP_GI_Dungeon.bLoadStartingItems` true (`.DungeonInstance` (`/Game/DCT/Blueprints/Core/BPFL_Singletons.GetDungeonGameInstance`)))))
    (if _bvalid
      (`/Game/DCT/Blueprints/Core/BP_PC_Dungeon.SetupUi` _dungeonplayercontroller)
      (`/Game/DCT/Blueprints/Core/BP_GI_Dungeon.StoreCharacterStats` (`.DungeonInstance` (`/Game/DCT/Blueprints/Core/BPFL_Singletons.GetDungeonGameInstance`)) (`self.PlayerCharacters`) false true)
      (if (`/Game/DCT/Blueprints/Core/BP_GI_Dungeon.bLoadStartingItems` (`.DungeonInstance` (`/Game/DCT/Blueprints/Core/BPFL_Singletons.GetDungeonGameInstance`)))
        (`self.LoadStartingItems`))
      (for _array_element (`self.PlayerCharacters`)
        (add `/Game/DCT/Blueprints/Core/BP_PlayerCharacter.OnKilled` _array_element (delegate `RunAfterCharacterKilled`))))))

(event `RunAfterCharacterKilled`
  (params (KilledCharacter :type "/Game/DCT/Blueprints/Core/BP_PlayerCharacter Object Reference"))
  ;[0 0 0] Begin Play
  (bind _bfoundlivingcharacters (`self.GetLivingPlayerCharacters`))
  (if (not _bfoundlivingcharacters)
    (`self.GameOver`)
    (`KismetSystemLibrary.Delay` 2.0)
    (`PlayerCameraManager.StartCameraFade` :`self` (`GameplayStatics.GetPlayerCameraManager` 0) :`ToAlpha` 1.0 :`Duration` 2.0 :`bHoldWhenFinished` true)
    (`KismetSystemLibrary.Delay` 2.0)
    (set `/Game/DCT/Blueprints/Core/BP_GI_Dungeon.TransitionTarget` "Load" (`.DungeonInstance` (`/Game/DCT/Blueprints/Core/BPFL_Singletons.GetDungeonGameInstance`)))
    (bind (_bvalid _savedlevel) (`/Game/DCT/Blueprints/Core/BP_GI_Dungeon.GetSavedLevel` (`.DungeonInstance` (`/Game/DCT/Blueprints/Core/BPFL_Singletons.GetDungeonGameInstance`))))
    (if _bvalid
      (`GameplayStatics.OpenLevel` (`KismetStringLibrary.Conv_StringToName` _savedlevel)))))

(event `AttemptUseItemEffect`
  (params (ItemType :type "DataTableRowHandle Structure") (ActivatingPlayerCharacter :type "/Game/DCT/Blueprints/Core/BP_PlayerCharacter Object Reference") (ResidingSlot :type "/Game/DCT/UserInterface/WBP_Slot Object Reference"))
  ;[0 0 0] Attempt Use Item Effect
  (bind (_bvalid _effect) (`self.GetItemEffectAndSpawnIfNeeded` ItemType))
  (if _bvalid
    (bind _ballvalid (`self.CheckSlottedItemUseRules` ResidingSlot true true))
    (if _ballvalid
      (`/Game/DCT/Blueprints/Effects/BP_Effect.UseEffect` _effect ActivatingPlayerCharacter ResidingSlot ItemType)
      (`/Engine/EditorBlueprintResources/StandardMacros.IsValid` (`/Game/DCT/UserInterface/WBP_Slot.SlottedItem` ResidingSlot)
        (:`Is Valid`
          (`self.OnItemUseDone`))))))

(event `/Game/DCT/Blueprints/Core/BPI_DungeonSingletons.SetActiveWidgetCharacter`
  (params (PlayerCharacter :type "/Game/DCT/Blueprints/Core/BP_PlayerCharacter Object Reference") (Subsheet :type "/Game/DCT/Data/ESubsheetSwitch Enum" :default "NewEnumerator0"))
  ;[0 0 0] Set Active Widget Character
  (if (== PlayerCharacter (`self.ActiveWidgetCharacter`))
    (bind _asbp_pc_dungeon (cast `/Game/DCT/Blueprints/Core/BP_PC_Dungeon` (`GameplayStatics.GetPlayerController` 0)))
    (bind _value (`BlueprintMapLibrary.Map_Find` (`/Game/DCT/Blueprints/Core/BP_PC_Dungeon.CharacterSheets` _asbp_pc_dungeon) (`self.ActiveWidgetCharacter`)))
    (`Widget.SetVisibility` _value (select `ESlateVisibility` (`Widget.GetVisibility` _value) :`Visible` "Hidden" :`Collapsed` "Visible" :`Hidden` "Visible" :`HitTestInvisible` "Hidden" :`SelfHitTestInvisible` "Hidden" :!type "ESlateVisibility Enum"))
    (else
      (set `self.ActiveWidgetCharacter` PlayerCharacter)
      (bind _asbp_pc_dungeon_2 (cast `/Game/DCT/Blueprints/Core/BP_PC_Dungeon` (`GameplayStatics.GetPlayerController` 0)))
      (bind _value_2 (`BlueprintMapLibrary.Map_Find` (`/Game/DCT/Blueprints/Core/BP_PC_Dungeon.CharacterSheets` _asbp_pc_dungeon_2) (`self.ActiveWidgetCharacter`)))
      (`WidgetSwitcher.SetActiveWidget` (`/Game/DCT/UserInterface/WBP_Layout.SheetSwitcher` (`/Game/DCT/Blueprints/Core/BP_PC_Dungeon.LayoutRef` _asbp_pc_dungeon_2)) _value_2)
      (`WidgetSwitcher.SetActiveWidgetIndex` (`/Game/DCT/UserInterface/WBP_CharacterSheet.CharacterWidgetSwitcher` _value_2) (`self.ActiveCharacterSheetWidgetIndex`))
      (`Widget.SetVisibility` _value_2 "Visible"))))

(event `/Game/DCT/Blueprints/Core/BPI_DungeonSingletons.SetActiveCharacterSheetWidgetIndex`
  (params (Index :type Integer))
  ;[0 0 0] Set Active Widget Character
  (set `self.ActiveCharacterSheetWidgetIndex` Index))

(event `RunItemSlotEffect`
  (params (bRemoved :type Boolean) (ItemWidget :type "/Game/DCT/UserInterface/WBP_Item Object Reference (by ref)") (Slot :type "/Game/DCT/UserInterface/WBP_Slot Object Reference") (bLoadingExisting :type Boolean))
  ;[0 0 0] Run Item Slot Effect
  (bind (_bvalid _effect) (`self.GetItemEffectAndSpawnIfNeeded` (`/Game/DCT/UserInterface/WBP_Item.ItemType` ItemWidget)))
  (if _bvalid
    (`/Game/DCT/Blueprints/Core/BPI_Interact.RunSlotEffect` _effect bRemoved Slot (`/Game/DCT/UserInterface/WBP_Slot.PlayerCharacterRef` Slot) ItemWidget bLoadingExisting)))

(event `/Game/DCT/Blueprints/Core/BPI_DungeonSingletons.CloseCharacterSheet`
  ;[0 0 0] Set Active Widget Character
  (bind _asbp_pc_dungeon (cast `/Game/DCT/Blueprints/Core/BP_PC_Dungeon` (`GameplayStatics.GetPlayerController` 0)))
  (`Widget.SetVisibility` (`BlueprintMapLibrary.Map_Find` (`/Game/DCT/Blueprints/Core/BP_PC_Dungeon.CharacterSheets` _asbp_pc_dungeon) (`self.ActiveWidgetCharacter`)) "Hidden"))

(fn `CheckItemSlotRules`
  (params (Item :type "/Game/DCT/UserInterface/WBP_Item Object Reference") (Slot :type "/Game/DCT/UserInterface/WBP_Slot Object Reference") (Interaction :type "/Game/DCT/Data/ESlotInteraction Enum" :default "NewEnumerator0"))
  (returns (bAllValid :type Boolean))
  (bind (_itemtype_datatable _itemtype_rowname) (break `DataTableRowHandle` (`/Game/DCT/UserInterface/WBP_Item.ItemType` Item)))
  (bind _item (`local.Item`))
  (bind _slot (`local.Slot`))
  (bind _returnvalue (`|GetDataTableRow` _itemtype_datatable _itemtype_rowname)
    (:`then`
      (for _array_element (`.SlotRules_147_6EF270EF4C10591630563DA882EC49EA` (break `/Game/DCT/Data/FItem` _returnvalue))
        (bind _slotrule (`self.GetSlotRuleOrCreateIfNeeded` _array_element))
        (switch `/Game/DCT/Data/ESlotInteraction` (`local.Interaction`)
          (:`NewEnumerator0`
            (bind (_ballowed _failmessage) (`/Game/DCT/Blueprints/SlotRules/BP_SlotRule.CheckIfCanPickup` _slotrule _item _slot))
            (if (not _ballowed)
              (message `/Game/DCT/Blueprints/Core/BPI_PlayerController.DisplayWarning` (`GameplayStatics.GetPlayerController` 0) (`KismetTextLibrary.Conv_StringToText` _failmessage))
              (return false)))
          (:`NewEnumerator1`
            (bind (_ballowed_2 _failmessage_2) (`/Game/DCT/Blueprints/SlotRules/BP_SlotRule.CheckIfCanPutInSlot` _slotrule _item _slot))
            (if (not _ballowed_2)
              (message `/Game/DCT/Blueprints/Core/BPI_PlayerController.DisplayWarning` (`GameplayStatics.GetPlayerController` 0) (`KismetTextLibrary.Conv_StringToText` _failmessage_2))
              (return false))))))
    (:`RowNotFound`
      _))
  (return true))

(fn `CheckSlottedItemUseRules`
  (params (Slot :type "/Game/DCT/UserInterface/WBP_Slot Object Reference") (bDisplayFailMessage :type Boolean) (bResolveConsequences :type Boolean))
  (returns (bAllValid :type Boolean))
  (bind _slotteditem (`/Game/DCT/UserInterface/WBP_Slot.SlottedItem` Slot))
  (bind _slot (`local.Slot`))
  (bind (_itemtype_datatable _itemtype_rowname) (break `DataTableRowHandle` (`/Game/DCT/UserInterface/WBP_Item.ItemType` _slotteditem)))
  (`/Engine/EditorBlueprintResources/StandardMacros.IsValid` Slot
    (:`Is Valid`
      (`/Engine/EditorBlueprintResources/StandardMacros.IsValid` _slotteditem
        (:`Is Valid`
          (bind _returnvalue (`|GetDataTableRow` _itemtype_datatable _itemtype_rowname)
            (:`then`
              (bind ((`UseRules_143_72BA77AF488F628BC07B81B4CC9F08E1` _userules)) (break `/Game/DCT/Data/FItem` _returnvalue))
              (for _array_element _userules
                (bind _userule (`self.GetUseRuleOrCreateIfNeeded` _array_element))
                (bind (_ballowed _failmessage) (`/Game/DCT/Blueprints/UseRules/BP_UseRule.CheckIfUseAllowed` _userule (`local.Slot`)))
                (if (not _ballowed)
                  (if (`local.bDisplayFailMessage`)
                    (message `/Game/DCT/Blueprints/Core/BPI_PlayerController.DisplayWarning` (`GameplayStatics.GetPlayerController` 0) (`KismetTextLibrary.Conv_StringToText` _failmessage)))
                  (return false)))
              (if (`local.bResolveConsequences`)
                (for _array_element_2 _userules
                  (bind _userule_2 (`self.GetUseRuleOrCreateIfNeeded` _array_element_2))
                  (`/Game/DCT/Blueprints/UseRules/BP_UseRule.ResolveUseConsequence` _userule_2 _slot)
                  (`/Engine/EditorBlueprintResources/StandardMacros.IsValid` (`/Game/DCT/UserInterface/WBP_Slot.SlottedItem` _slot)
                    (:`Is Not Valid`
                      (return true))))
                (return true)
                (else
                  (return true))))
            (:`RowNotFound`
              (return false))))
        (:`Is Not Valid`
          (return false))))
    (:`Is Not Valid`
      (return false))))

(fn `ConstructAndSetupDefaultPlayerCharacters`
  (returns (PlayerCharacters :type "Array of /Game/DCT/Blueprints/Core/BP_PlayerCharacter Object Reference"))
  (locals (LocalPlayerCharacters :type "Array of /Game/DCT/Blueprints/Core/BP_PlayerCharacter Object Reference"))
  (bind _outrownames (`DataTableFunctionLibrary.GetDataTableRowNames` "/Game/DCT/Data/DT_DefaultCharacters.DT_DefaultCharacters"))
  (for _array_element _outrownames
    (bind _returnvalue (`|GetDataTableRow` "/Game/DCT/Data/DT_DefaultCharacters.DT_DefaultCharacters" _array_element)
      (:`then`
        (bind _returnvalue_2 (`|GenericCreateObject` self "/Game/DCT/Blueprints/Core/BP_PlayerCharacter.BP_PlayerCharacter_C" (break `/Game/DCT/Data/FCharacterData` _returnvalue) (`.Portrait_9_8CBB15404210CA1786058AA8FD0D7E5F` (break `/Game/DCT/Data/FCharacterData` _returnvalue)) (`.Race_65_6D25AA894CB86A15A75E938BB31E235A` (break `/Game/DCT/Data/FCharacterData` _returnvalue)) (`.Class_66_822D082440D4C80CEFF258BD1CDAF23B` (break `/Game/DCT/Data/FCharacterData` _returnvalue)) (`.BaseStats_69_FFBD65734BA4A4AD245D92B5DAF2B35B` (break `/Game/DCT/Data/FCharacterData` _returnvalue)) (`.CurrentStats_70_274565BC4038371455CBC38BAF2579DC` (break `/Game/DCT/Data/FCharacterData` _returnvalue))))
        (`/Game/DCT/Blueprints/Core/BP_PlayerCharacter.SetupStats` _returnvalue_2 (`/Game/DCT/Blueprints/Core/BP_GI_Dungeon.StatTags` (`.DungeonInstance` (`/Game/DCT/Blueprints/Core/BPFL_Singletons.GetDungeonGameInstance`))))
        (`KismetArrayLibrary.Array_Add` (`local.LocalPlayerCharacters`) _returnvalue_2))))
  (return (`local.LocalPlayerCharacters`)))

(fn `ConstructStoredPlayerCharacters`
  (params (PlayerCharacterData :type "Array of /Game/DCT/Data/FCharacterData Structure"))
  (returns (PlayerCharacters :type "Array of /Game/DCT/Blueprints/Core/BP_PlayerCharacter Object Reference"))
  (locals (LocalPlayerCharacters :type "Array of /Game/DCT/Blueprints/Core/BP_PlayerCharacter Object Reference"))
  (for _array_element PlayerCharacterData
    (bind ((`Name_2_F56A052F4007F06EF30B3CBA23222C90` _name) (`Portrait_9_8CBB15404210CA1786058AA8FD0D7E5F` _portrait) (`Race_65_6D25AA894CB86A15A75E938BB31E235A` _race) (`Class_66_822D082440D4C80CEFF258BD1CDAF23B` _class) (`BaseStats_69_FFBD65734BA4A4AD245D92B5DAF2B35B` _basestats) (`CurrentStats_70_274565BC4038371455CBC38BAF2579DC` _currentstats)) (break `/Game/DCT/Data/FCharacterData` _array_element))
    (bind _returnvalue (`|GenericCreateObject` self "/Game/DCT/Blueprints/Core/BP_PlayerCharacter.BP_PlayerCharacter_C" _name _portrait _race _class _basestats _currentstats))
    (`KismetArrayLibrary.Array_Add` (`local.LocalPlayerCharacters`) _returnvalue))
  (return (`local.LocalPlayerCharacters`)))

(fn `GameOver`
  (bind _returnvalue (`GameplayStatics.GetPlayerController` 0))
  (`self.DisableInput` (`GameplayStatics.GetPlayerPawn` 0) _returnvalue)
  (bind _returnvalue_2 (`|CreateWidget` "/Game/DCT/UserInterface/WBP_GameOver.WBP_GameOver_C" _returnvalue))
  (`UserWidget.AddToViewport` _returnvalue_2 0)
  (return))

(fn `GetActiveCharacterSheetWidgetIndex`
  (returns (Index :type Integer))
  (return (`self.ActiveCharacterSheetWidgetIndex`)))

(fn `GetActiveWidgetCharacter`
  (returns (bValid :type Boolean) (PlayerCharacterRef :type "/Game/DCT/Blueprints/Core/BP_PlayerCharacter Object Reference"))
  (bind _activewidgetcharacter (`self.ActiveWidgetCharacter`))
  (return (`KismetSystemLibrary.IsValid` _activewidgetcharacter) _activewidgetcharacter))

(fn `GetItemEffectAndSpawnIfNeeded`
  (params (ItemType :type "DataTableRowHandle Structure (by ref)"))
  (returns (bValid :type Boolean) (Effect :type "/Game/DCT/Blueprints/Effects/BP_Effect Object Reference"))
  (bind (_datatable _rowname) (break `DataTableRowHandle` ItemType))
  (`/Engine/EditorBlueprintResources/StandardMacros.IsValid` _datatable
    (:`Is Valid`
      (bind _returnvalue (`|GetDataTableRow` _datatable _rowname)
        (:`then`
          (bind ((`EffectBlueprint_66_A36C56C54EACFD9923F63FACFE71BEC5` _effectblueprint)) (break `/Game/DCT/Data/FItem` _returnvalue))
          (bind (_value _returnvalue_2) (`BlueprintMapLibrary.Map_Find` (`self.EffectClasses`) _effectblueprint))
          (if _returnvalue_2
            (return (`KismetSystemLibrary.IsValid` _value) _value)
            (else
              (bind _returnvalue_3 (`|SpawnActorFromClass` _effectblueprint (`KismetMathLibrary.MakeTransform` (0.0 0.0 0.0)) "AlwaysSpawn" "SelectDefaultAtRuntime" null (struct) null))
              (`BlueprintMapLibrary.Map_Add` (`self.EffectClasses`) _effectblueprint _returnvalue_3)
              (return (`KismetSystemLibrary.IsValid` _returnvalue_3) _returnvalue_3))))
        (:`RowNotFound`
          _)))
    (:`Is Not Valid`
      _))
  (return false null))

(fn `GetLivingPlayerCharacters`
  (returns (bFoundLivingCharacters :type Boolean) (LivingPlayerCharacters :type "Array of /Game/DCT/Blueprints/Core/BP_PlayerCharacter Object Reference"))
  (locals (LocalCharacters :type "Array of /Game/DCT/Blueprints/Core/BP_PlayerCharacter Object Reference"))
  (for _array_element (`self.PlayerCharacters`)
    (if (not (`/Game/DCT/Blueprints/Core/BP_PlayerCharacter.bDead` _array_element))
      (`KismetArrayLibrary.Array_Add` (`local.LocalCharacters`) _array_element)))
  (return (> (`KismetArrayLibrary.Array_Length` (`local.LocalCharacters`)) 0) (`local.LocalCharacters`)))

(fn `GetRandomLivingPlayerCharacter`
  (returns (bValid :type Boolean) (RandomPlayerCharacter :type "/Game/DCT/Blueprints/Core/BP_PlayerCharacter Object Reference"))
  (bind (_bfoundlivingcharacters _livingplayercharacters) (`self.GetLivingPlayerCharacters`))
  (if _bfoundlivingcharacters
    (return true (`|GetArrayItem` _livingplayercharacters (`KismetMathLibrary.RandomIntegerInRange` 0 (`KismetArrayLibrary.Array_LastIndex` _livingplayercharacters))))
    (else
      (return false null))))

(fn `GetSlotRuleOrCreateIfNeeded`
  (params (SlotRuleClass :type "/Game/DCT/Blueprints/SlotRules/BP_SlotRule Class Reference (by ref)"))
  (returns (SlotRule :type "/Game/DCT/Blueprints/SlotRules/BP_SlotRule Object Reference"))
  (bind (_value _returnvalue) (`BlueprintMapLibrary.Map_Find` (`self.SlotRules`) SlotRuleClass))
  (if _returnvalue
    (return _value)
    (else
      (bind _returnvalue_2 (`|GenericCreateObject` self (`local.SlotRuleClass`)))
      (`BlueprintMapLibrary.Map_Add` (`self.SlotRules`) (`local.SlotRuleClass`) _returnvalue_2)
      (return _returnvalue_2))))

(fn `GetUseRuleOrCreateIfNeeded`
  (params (UseRuleClass :type "/Game/DCT/Blueprints/UseRules/BP_UseRule Class Reference (by ref)"))
  (returns (UseRule :type "/Game/DCT/Blueprints/UseRules/BP_UseRule Object Reference"))
  (bind (_value _returnvalue) (`BlueprintMapLibrary.Map_Find` (`self.UseRules`) UseRuleClass))
  (if _returnvalue
    (return _value)
    (else
      (bind _returnvalue_2 (`|GenericCreateObject` self (`local.UseRuleClass`)))
      (`BlueprintMapLibrary.Map_Add` (`self.UseRules`) (`local.UseRuleClass`) _returnvalue_2)
      (return _returnvalue_2))))

(fn `IsCharacterSheetOpen`
  (returns (bIsOpen :type Boolean))
  (bind _asbp_pc_dungeon (cast `/Game/DCT/Blueprints/Core/BP_PC_Dungeon` (`GameplayStatics.GetPlayerController` 0)))
  (bind (_value _returnvalue) (`BlueprintMapLibrary.Map_Find` (`/Game/DCT/Blueprints/Core/BP_PC_Dungeon.CharacterSheets` _asbp_pc_dungeon) (`self.ActiveWidgetCharacter`)))
  (if _returnvalue
    (return (`Widget.IsVisible` _value))
    (else
      (return false))))

(fn `LoadStartingItems`
  (locals (EmptyMap :type "Map of Integer to /Game/DCT/Data/FItemSave Structure"))
  (for _array_element (`self.PlayerCharacters`)
    (bind (_characterclass_datatable _characterclass_rowname) (break `DataTableRowHandle` (`/Game/DCT/Blueprints/Core/BP_PlayerCharacter.CharacterClass` _array_element)))
    (bind _returnvalue (`|GetDataTableRow` _characterclass_datatable _characterclass_rowname)
      (:`then`
        (bind _wbp_inventory (`/Game/DCT/UserInterface/WBP_CharacterSheet.WBP_Inventory` (`BlueprintMapLibrary.Map_Find` (`/Game/DCT/Blueprints/Core/BP_PC_Dungeon.CharacterSheets` (`.DungeonPlayerController` (`/Game/DCT/Blueprints/Core/BPFL_Singletons.GetDungeonPlayerController`))) _array_element)))
        (bind ((`Stats_36_3907E16340AE15C1244A959B2CFC6004` _stats) (`StartingInventory_32_15D910DB42BA4A4269006EABB9BC5040` _startinginventory) (`StartingEquipment_35_0C3733DB407ADA3A42720F9BFC2C004A` _startingequipment)) (break `/Game/DCT/Data/FStatsMap` _returnvalue))
        (`/Game/DCT/UserInterface/WBP_Inventory.LoadItems` _wbp_inventory _startinginventory (`local.EmptyMap`) true false)
        (`/Game/DCT/UserInterface/WBP_Inventory.LoadEquipmentByType` _wbp_inventory _startingequipment true))))
  (set `/Game/DCT/Blueprints/Core/BP_GI_Dungeon.bLoadStartingItems` false (`.DungeonInstance` (`/Game/DCT/Blueprints/Core/BPFL_Singletons.GetDungeonGameInstance`)))
  (return))

(fn `RewardExperience`
  (params (Experience :type "Float (double-precision)"))
  (bind (_bfoundlivingcharacters _livingplayercharacters) (`self.GetLivingPlayerCharacters`))
  (for _array_element _livingplayercharacters
    (`/Game/DCT/Blueprints/Core/BP_PlayerCharacter.ModifyStat` _array_element Experience (struct :`TagName` "Stat.Experience") false "NewEnumerator0" true false))
  (return))

(fn `UserConstructionScript`)