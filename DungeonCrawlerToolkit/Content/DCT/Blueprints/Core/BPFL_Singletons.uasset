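; Blueprint function library giving global access to the dungeon game's core objects, each returned with a Valid flag.
; Getters cast the game mode, game state, game instance, and player 0's controller and pawn, while the dungeon manager is found by actor class.
; Two helpers build on them: tag display names from the game instance's map, and stat text formatted per the game state's formats, both with fallbacks.
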(fn `GetDungeonGameInstance`
  (returns (bValid :type Boolean) (DungeonInstance :type "/Game/DCT/Blueprints/Core/BP_GI_Dungeon Object Reference"))
  (bind _asbp_gi_dungeon (cast `/Game/DCT/Blueprints/Core/BP_GI_Dungeon` (`GameplayStatics.GetGameInstance` null))
    (:`then`
      (return true _asbp_gi_dungeon))
    (:`CastFailed`
      (return false null))))

(fn `GetDungeonGameMode`
  (returns (bValid :type Boolean) (DungeonMode :type "/Game/DCT/Blueprints/Core/BP_Dungeon Object Reference"))
  (bind _asbp_dungeon (cast `/Game/DCT/Blueprints/Core/BP_Dungeon` (`GameplayStatics.GetGameMode` null))
    (:`then`
      (return true _asbp_dungeon))
    (:`CastFailed`
      (return false null))))

(fn `GetDungeonGameState`
  (returns (bValid :type Boolean) (DungeonState :type "/Game/DCT/Blueprints/Core/BP_Dungeon_State Object Reference"))
  (bind _asbp_dungeon_state (cast `/Game/DCT/Blueprints/Core/BP_Dungeon_State` (`GameplayStatics.GetGameState` null))
    (:`then`
      (return true _asbp_dungeon_state))
    (:`CastFailed`
      (return false null))))

(fn `GetDungeonManager`
  (returns (bValid :type Boolean) (DungeonManager :type "/Game/DCT/Blueprints/Core/BP_DungeonManager Object Reference"))
  (bind _returnvalue (`GameplayStatics.GetActorOfClass` null "/Game/DCT/Blueprints/Core/BP_DungeonManager.BP_DungeonManager_C"))
  (return (`KismetSystemLibrary.IsValid` _returnvalue) _returnvalue))

(fn `GetDungeonPawn`
  (returns (bValid :type Boolean) (DungeonPawn :type "/Game/DCT/Blueprints/Core/BP_DungeonPawn Object Reference"))
  (bind _asbp_dungeon_pawn (cast `/Game/DCT/Blueprints/Core/BP_DungeonPawn` (`GameplayStatics.GetPlayerPawn` null))
    (:`then`
      (return true _asbp_dungeon_pawn))
    (:`CastFailed`
      (return false null))))

(fn `GetDungeonPlayerController`
  (returns (bValid :type Boolean) (DungeonPlayerController :type "/Game/DCT/Blueprints/Core/BP_PC_Dungeon Object Reference"))
  (bind _asbp_pc_dungeon (cast `/Game/DCT/Blueprints/Core/BP_PC_Dungeon` (`GameplayStatics.GetPlayerController` null))
    (:`then`
      (return true _asbp_pc_dungeon))
    (:`CastFailed`
      (return false null))))

(fn `GetFormattedStatValueText`
  (params (Stat :type "GameplayTag Structure") (Value :type "Float (double-precision)"))
  (returns (FormattedText :type Text))
  (bind (_bvalid _dungeonstate) (`self.GetDungeonGameState` null))
  (bind (_value _returnvalue) (`BlueprintMapLibrary.Map_Find` (`/Game/DCT/Blueprints/Core/BP_Dungeon_State.StatFormats` _dungeonstate) (`local.Stat`)))
  (if _bvalid
    (if _returnvalue
      (switch `/Game/DCT/Data/EStatFormat` _value
        (:`NewEnumerator0`
          _)
        (:`NewEnumerator1`
          (return (`KismetTextLibrary.Conv_StringToText` (`KismetStringLibrary.Concat_StrStr` (`KismetStringLibrary.Conv_IntToString` (`KismetMathLibrary.Round` (* (`local.Value`) 100.0))) "%"))))
        (:`NewEnumerator2`
          (return (`KismetTextLibrary.Conv_DoubleToText` (`local.Value`) "HalfToEven"))))))
  (return (`KismetTextLibrary.Conv_IntToText` (`KismetMathLibrary.Round` (`local.Value`)))))

(fn `GetTagFriendlyName`
  (params (GameplayTag :type "GameplayTag Structure (by ref)"))
  (returns (FriendlyName :type String))
  (bind (_bvalid _dungeoninstance) (`self.GetDungeonGameInstance` null))
  (bind (_value _returnvalue) (`BlueprintMapLibrary.Map_Find` (`/Game/DCT/Blueprints/Core/BP_GI_Dungeon.FriendlyTagNames` _dungeoninstance) (`local.GameplayTag`)))
  (if _bvalid
    (if _returnvalue
      (return _value)
      (else
        _)))
  (return (`/Game/DCT/Blueprints/Core/BPFL_Dungeon.GetLowestLevelTagName` (`local.GameplayTag`))))