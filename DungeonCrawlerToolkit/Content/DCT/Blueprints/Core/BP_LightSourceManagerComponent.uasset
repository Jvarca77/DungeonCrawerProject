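; Actor component that manages competing light settings for the Point Light on its owning actor, showing only the most intense one.
; It keeps a list of light sources, seeded on BeginPlay with default properties, that grows and shrinks through add and remove events.
; Each change rescans the list and copies the brightest entry's intensity, color and attenuation radius onto the light, without blending.
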(event `self.ReceiveBeginPlay`
  (set `self.LightReference` (`Actor.GetComponentByClass` (`self.GetOwner`) "/Script/Engine.PointLightComponent"))
  (`KismetArrayLibrary.Array_Add` (`self.LightSources`) (`self.DefaultLightProperties`)))

(event `AddLightSource`
  (params (LightSource :type "/Game/DCT/Blueprints/Core/FLightSource Structure"))
  (`self.LightReference`
    (:`then`
      _)
    (:`else`
      (set `self.LightReference` (`Actor.GetComponentByClass` (`self.GetOwner`) "/Script/Engine.PointLightComponent"))))
  (`KismetArrayLibrary.Array_Add` (`self.LightSources`) LightSource)
  (`self.ChooseDominantLight`))

(event `RemoveLightSource`
  (params (LightSource :type "/Game/DCT/Blueprints/Core/FLightSource Structure (by ref)"))
  (bind _returnvalue (`KismetArrayLibrary.Array_Find` (`self.LightSources`) LightSource))
  (if (>= _returnvalue 0)
    (`KismetArrayLibrary.Array_Remove` (`self.LightSources`) _returnvalue)
    (`self.ChooseDominantLight`)))

(fn `ChooseDominantLight`
  (locals (LocalMaxIntensity :type "Float (double-precision)"))
  (for _array_element (`self.LightSources`)
    (if (> (break `/Game/DCT/Blueprints/Core/FLightSource` _array_element) (`local.LocalMaxIntensity`))
      (bind _output_get (set `local.LocalMaxIntensity` (break `/Game/DCT/Blueprints/Core/FLightSource` _array_element)))
      (`LightComponent.SetIntensity` (`self.LightReference`) _output_get)
      (`LightComponent.SetLightColor` (`self.LightReference`) (`.Color_5_D5FAA6D64C15BBD7D89C21BC4DB64733` (break `/Game/DCT/Blueprints/Core/FLightSource` _array_element)) true)
      (`LocalLightComponent.SetAttenuationRadius` (`self.LightReference`) (`.Attenuation_8_EA38330A4C22BB978AFE9B906B9EDAF3` (break `/Game/DCT/Blueprints/Core/FLightSource` _array_element)))))
  (return))