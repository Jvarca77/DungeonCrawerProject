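; Player controller for the dungeon crawler, owning the party HUD, input and cursor-held item or power.
; SetupUi waits for the game state, builds a character sheet and mini portrait per party member, then loads saved inventories.
; Input toggles sheets and menu, flags stack splitting and maps keys to slots across portraits.
; The held widget follows the mouse; ScreenInteract tries interfaced actors, otherwise drops items on adjacent surfaces or returns them.
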(event `self.ReceiveBeginPlay`
  ;[0 0 0] Setup Input
  (`EnhancedInputSubsystemInterface.AddMappingContext` (subsystem `EnhancedInputLocalPlayerSubsystem`) "/Game/DCT/Input/IMC_DCT.IMC_DCT" 0 (struct))
  (`Widget.SetVisibility` (`/Game/DCT/UserInterface/WBP_Layout.WBP_MoveGrid` (`self.LayoutRef`)) (select `bool` (`/Game/DCT/Blueprints/Core/BP_GI_Dungeon.bMovementArrows` (`.DungeonInstance` (`/Game/DCT/Blueprints/Core/BPFL_Singletons.GetDungeonGameInstance`))) :`false` "Collapsed" :`true` "Visible" :!type "ESlateVisibility Enum")))

(event `SetupUi`
  (bind (_bvalid _dungeonstate) (`/Game/DCT/Blueprints/Core/BPFL_Singletons.GetDungeonGameState`))
  (bind (_bvalid_2 _dungeonstate_2) (`/Game/DCT/Blueprints/Core/BPFL_Singletons.GetDungeonGameState`))
  (bind _output (`|GetArrayItem` (`/Game/DCT/Blueprints/Core/BP_Dungeon_State.PlayerCharacters` _dungeonstate_2)))
  ;[0 0 0] Setup UI
  (bind _returnvalue (`|CreateWidget` "/Game/DCT/UserInterface/WBP_Layout.WBP_Layout_C" self))
  (bind _output_get (set `self.LayoutRef` _returnvalue))
  (`UserWidget.AddToViewport` _output_get 0)
  (bind _returnvalue_2 (`|CreateWidget` "/Game/DCT/UserInterface/WBP_WarningDisplay.WBP_WarningDisplay_C" self))
  (bind _output_get_2 (set `self.WarningDisplayRef` _returnvalue_2))
  (`UserWidget.AddToViewport` _output_get_2 0)
  (`/Game/DCT/Blueprints/Core/BPML_Utility.DelayWhile` (not _bvalid)
    (:`Continue`
      (for (_array_element _array_index) (`/Game/DCT/Blueprints/Core/BP_Dungeon_State.PlayerCharacters` _dungeonstate)
        (`self.SetupPlayerCharacterUi` _array_element _array_index))
      (message `/Game/DCT/Blueprints/Core/BPI_DungeonSingletons.SetActiveWidgetCharacter` _dungeonstate_2 _output "NewEnumerator0")
      (`/Game/DCT/UserInterface/WBP_CharacterSheet.ToggleSubsheets` (`/Game/DCT/Blueprints/Core/BP_PlayerCharacter.CharacterSheetRef` _output) 0)
      (`self.LoadCharacterItems`))))

(event `EnhancedInput|/Game/DCT/Input/IA_Inventory`
  (params (ActionValue :type Boolean) (ElapsedSeconds :type "Float (double-precision)") (TriggeredSeconds :type "Float (double-precision)") (InputAction :type "InputAction Object Reference" :default "/Game/DCT/Input/IA_Inventory.IA_Inventory"))
  ;[0 0 0] UI input
  (:`Started`
    (bind (_bvalid _playercharacterref) (message `/Game/DCT/Blueprints/Core/BPI_DungeonSingletons.GetActiveWidgetCharacter` (`GameplayStatics.GetGameState`)))
    (`/Game/DCT/UserInterface/WBP_CharacterSheet.ToggleSubsheets` (`BlueprintMapLibrary.Map_Find` (`self.CharacterSheets`) _playercharacterref) 0)))

(event `EnhancedInput|/Game/DCT/Input/IA_Character`
  (params (ActionValue :type Boolean) (ElapsedSeconds :type "Float (double-precision)") (TriggeredSeconds :type "Float (double-precision)") (InputAction :type "InputAction Object Reference" :default "/Game/DCT/Input/IA_Character.IA_Character"))
  ;[0 0 0] UI input
  (:`Started`
    (bind (_bvalid _playercharacterref) (message `/Game/DCT/Blueprints/Core/BPI_DungeonSingletons.GetActiveWidgetCharacter` (`GameplayStatics.GetGameState`)))
    (`/Game/DCT/UserInterface/WBP_CharacterSheet.ToggleSubsheets` (`BlueprintMapLibrary.Map_Find` (`self.CharacterSheets`) _playercharacterref) 1)))

(event `EnhancedInput|/Game/DCT/Input/IA_Menu`
  (params (ActionValue :type Boolean) (ElapsedSeconds :type "Float (double-precision)") (TriggeredSeconds :type "Float (double-precision)") (InputAction :type "InputAction Object Reference" :default "/Game/DCT/Input/IA_Menu.IA_Menu"))
  (bind _wbp_menu (`/Game/DCT/UserInterface/WBP_Layout.WBP_Menu` (`self.LayoutRef`)))
  ;[0 0 0] Open/Close Menu
  (:`Started`
    (bind _bisopen (message `/Game/DCT/Blueprints/Core/BPI_DungeonSingletons.IsCharacterSheetOpen` (`GameplayStatics.GetGameState`)))
    (if _bisopen
      (message `/Game/DCT/Blueprints/Core/BPI_DungeonSingletons.CloseCharacterSheet` (`GameplayStatics.GetGameState`))
      (else
        (`Widget.SetVisibility` _wbp_menu (select `ESlateVisibility` (`Widget.GetVisibility` _wbp_menu) :`Visible` "Hidden" :`Collapsed` "Hidden" :`Hidden` "SelfHitTestInvisible" :`HitTestInvisible` "Hidden" :`SelfHitTestInvisible` "Hidden" :!type "ESlateVisibility Enum"))))))

(event `EnhancedInput|/Game/DCT/Input/IA_Powers`
  (params (ActionValue :type Boolean) (ElapsedSeconds :type "Float (double-precision)") (TriggeredSeconds :type "Float (double-precision)") (InputAction :type "InputAction Object Reference" :default "/Game/DCT/Input/IA_Powers.IA_Powers"))
  ;[0 0 0] UI input
  (:`Started`
    (bind (_bvalid _playercharacterref) (message `/Game/DCT/Blueprints/Core/BPI_DungeonSingletons.GetActiveWidgetCharacter` (`GameplayStatics.GetGameState`)))
    (`/Game/DCT/UserInterface/WBP_CharacterSheet.ToggleSubsheets` (`BlueprintMapLibrary.Map_Find` (`self.CharacterSheets`) _playercharacterref) 2)))

(event `self.ReceiveTick`
  (params (DeltaSeconds :type "Float (single-precision)"))
  ;[0 0 0] Move mouse widget on tick
  (`/Engine/EditorBlueprintResources/StandardMacros.IsValid` (`self.MouseFollowWidget`)
    (:`Is Valid`
      (bind _returnvalue (`WidgetLayoutLibrary.GetMousePositionOnViewport`))
      (`Widget.SetRenderTransform` (`self.MouseFollowWidget`) (make `WidgetTransform` (`KismetMathLibrary.MakeVector2D` (`KismetMathLibrary.BreakVector2D` _returnvalue) (`.Y` (`KismetMathLibrary.BreakVector2D` _returnvalue)))))
      (`Widget.SetVisibility` (`self.MouseFollowWidget`) (select `bool` (`.ReturnValue` (`self.GetMousePosition`)) :`false` "Hidden" :`true` "HitTestInvisible" :!type "ESlateVisibility Enum")))))

(event `EnhancedInput|/Game/DCT/Input/IA_StackSplit`
  (params (ActionValue :type Boolean) (ElapsedSeconds :type "Float (double-precision)") (TriggeredSeconds :type "Float (double-precision)") (InputAction :type "InputAction Object Reference" :default "/Game/DCT/Input/IA_StackSplit.IA_StackSplit"))
  ;[0 0 0] UI input
  (:`Started`
    (set `self.bStackSplitPressed` true))
  (:`Canceled`
    (set `self.bStackSplitPressed` false :!label _label))
  (:`Completed`
    (goto _label)))

(event `EnhancedInput|/Game/DCT/Input/IA_UseSlot`
  (params (ActionValue :type "Float (double-precision)") (ElapsedSeconds :type "Float (double-precision)") (TriggeredSeconds :type "Float (double-precision)") (InputAction :type "InputAction Object Reference" :default "/Game/DCT/Input/IA_UseSlot.IA_UseSlot"))
  ;[0 0 0] UI input
  (:`Started`
    (`self.ActivateSlotFromKeyboardInput` (`KismetMathLibrary.FTrunc` ActionValue))))

(event `/Game/DCT/Blueprints/Core/BPI_PlayerController.SetMouseWidget`
  (params (Widget :type "/Game/DCT/UserInterface/WBP_Item Object Reference"))
  (bind _wbp_helditemdisplay (`/Game/DCT/UserInterface/WBP_Layout.WBP_HeldItemDisplay` (`self.LayoutRef`)))
  ;[0 0 0] Set Mouse Widget
  (bind _output_get (set `self.MouseFollowWidget` Widget))
  (`/Engine/EditorBlueprintResources/StandardMacros.IsValid` _output_get
    (:`Is Valid`
      (`self.UpdateMouseFollowWidgetInViewport`)
      (`KismetSystemLibrary.Delay` 0.0)
      (`/Game/DCT/UserInterface/WBP_HeldItemDisplay.UpdateHeldItemDisplay` _wbp_helditemdisplay (`/Game/DCT/UserInterface/WBP_Item.GetItemName` (`self.MouseFollowWidget`))))
    (:`Is Not Valid`
      (`/Game/DCT/UserInterface/WBP_HeldItemDisplay.UpdateHeldItemDisplay` _wbp_helditemdisplay "None"))))

(event `/Game/DCT/Blueprints/Core/BPI_PlayerController.DisplayWarning`
  (params (MessageText :type Text))
  ;[0 0 0] Error Message Display
  (`/Game/DCT/UserInterface/WBP_WarningDisplay.DisplayWarning` (`self.WarningDisplayRef`) MessageText))

(event `ScreenInteract`
  (bind _mousefollowwidget (`self.MouseFollowWidget`))
  (bind (_bblockinghit _binitialoverlap _time _distance _location) (`GameplayStatics.BreakHitResult` (`self.ScreenInteractResult`)))
  ;[0 0 0] Screen Interact
  (bind _output_get (set `self.ScreenInteractResult` (`self.GetHitResultUnderCursorByChannel` "TraceTypeQuery1")))
  (bind (_bblockinghit_2 _binitialoverlap_2 _time_2 _distance_2 _location_2 _impactpoint _normal _impactnormal _physmat _hitactor) (`GameplayStatics.BreakHitResult` _output_get))
  (`/Engine/EditorBlueprintResources/StandardMacros.IsValid` _hitactor
    (:`Is Valid`
      (if (`KismetSystemLibrary.DoesImplementInterface` _hitactor "/Game/DCT/Blueprints/Core/BPI_Interact.BPI_Interact_C")
        (bind _bsuccess (message `/Game/DCT/Blueprints/Core/BPI_Interact.AttemptInteract` _hitactor (`GameplayStatics.GetPlayerPawn` 0)))
        (if _bsuccess
          (`/Engine/EditorBlueprintResources/StandardMacros.IsValid` (`self.MouseFollowWidget`)
            (:`Is Valid`
              (bind _btrue (`/Game/DCT/UserInterface/WBP_Item.IsPower` (`self.MouseFollowWidget`)))
              (if _btrue
                (`self.ClearMouseFollowWidget` :!label _label_2))))
          (else
            (`/Engine/EditorBlueprintResources/StandardMacros.IsValid` (`self.MouseFollowWidget`) :!label _label_3
              (:`Is Valid`
                (bind _btrue_2 (`/Game/DCT/UserInterface/WBP_Item.IsPower` (`self.MouseFollowWidget`)))
                (if _btrue_2
                  (goto _label_2)
                  (else
                    (bind _returnvalue (`self.GetComponentByClass` _hitactor "/Script/Engine.StaticMeshComponent"))
                    (`/Engine/EditorBlueprintResources/StandardMacros.IsValid` _returnvalue
                      (:`Is Valid`
                        (switch `ECollisionResponse` (`PrimitiveComponent.GetCollisionResponseToChannel` _returnvalue "ECC_GameTraceChannel2")
                          (:`ECR_Block`
                            (if (`GameplayStatics.BreakHitResult` (`self.ScreenInteractResult`))
                              (if (`/Game/DCT/Blueprints/Core/BP_DungeonManager.IsAdjacent` (`.DungeonManager` (`/Game/DCT/Blueprints/Core/BPFL_Singletons.GetDungeonManager`)) (`self.K2_GetActorLocation` (`GameplayStatics.GetPlayerPawn` 0)) _location)
                                (`|SpawnActorFromClass` "/Game/DCT/Blueprints/Items/BP_Item.BP_Item_C" (`KismetMathLibrary.Conv_VectorToTransform` (+ _location (0.0 0.0 10.0))) "AdjustIfPossibleButAlwaysSpawn" "OverrideRootScale" null (`/Game/DCT/UserInterface/WBP_Item.Amount` _mousefollowwidget) (make `DataTableRowHandle` "/Game/DCT/Data/DT_Items.DT_Items" (`/Game/DCT/UserInterface/WBP_Item.GetItemName` _mousefollowwidget)) true null)
                                (`self.ClearMouseFollowWidget`)
                                (else
                                  (`/Game/DCT/UserInterface/WBP_Item.PlaceBackInLastSlotIfValid` (`self.MouseFollowWidget`))))
                              (else
                                (`/Game/DCT/UserInterface/WBP_Item.PlaceBackInLastSlotIfValid` (`self.MouseFollowWidget`))))))))))))))
        (else
          (goto _label_3))))
    (:`Is Not Valid`
      (goto _label_3))))

(fn `ActivateSlotFromKeyboardInput`
  (params (InputNumber :type Integer))
  (for (_array_element _array_index) (`PanelWidget.GetAllChildren` (`/Game/DCT/UserInterface/WBP_Layout.MiniCharacterPanel` (`self.LayoutRef`)))
    (bind _aswbp_mini_character (cast `/Game/DCT/UserInterface/WBP_MiniCharacter` _array_element))
    (bind _allslots (`/Game/DCT/UserInterface/WBP_MiniCharacter.GetAllSlots` _aswbp_mini_character))
    (for (_array_element_2 _array_index_2) _allslots
      (if (== (+ (+ _array_index_2 (* (`KismetArrayLibrary.Array_Length` _allslots) _array_index)) 1) (`local.InputNumber`))
        (`/Game/DCT/UserInterface/WBP_Slot.InteractWithSlot` _array_element_2)
        (return))))
  (return))

(fn `ClearMouseFollowWidget`
  (bind _mousefollowwidget (`self.MouseFollowWidget`)
    (:`then`
      (`Widget.RemoveFromParent` _mousefollowwidget)
      (`/Game/DCT/Blueprints/Core/BPI_PlayerController.SetMouseWidget` null)
      (return))
    (:`else`
      (return))))

(fn `GetMouseWidget`
  (returns (Widget :type "/Game/DCT/UserInterface/WBP_Item Object Reference"))
  (return (`self.MouseFollowWidget`)))

(fn `IsStackSplitPressed`
  (returns (bTrue :type Boolean))
  (return (`self.bStackSplitPressed`)))

(fn `LoadCharacterItems`
  (bind (_bvalid _playercharacterdata) (`/Game/DCT/Blueprints/Core/BP_GI_Dungeon.GetSavedCharacters` (`.DungeonInstance` (`/Game/DCT/Blueprints/Core/BPFL_Singletons.GetDungeonGameInstance`))))
  (if _bvalid
    (bind _values (`BlueprintMapLibrary.Map_Values` (`self.CharacterSheets`)))
    (for (_array_element _array_index) _values
      (bind (_output_name _output_portrait _output_inventory _output_equipment) (break `/Game/DCT/Data/FCharacterData` (`|GetArrayItem` _playercharacterdata _array_index)))
      (`/Game/DCT/UserInterface/WBP_Inventory.LoadItems` (`/Game/DCT/UserInterface/WBP_CharacterSheet.WBP_Inventory` _array_element) _output_inventory _output_equipment true true))
    (return)))

(fn `SetupPlayerCharacterUi`
  (params (PlayerCharacter :type "/Game/DCT/Blueprints/Core/BP_PlayerCharacter Object Reference") (CharacterIndex :type Integer))
  (bind _characterindex (`local.CharacterIndex`))
  (bind _returnvalue (`|CreateWidget` "/Game/DCT/UserInterface/WBP_CharacterSheet.WBP_CharacterSheet_C" self PlayerCharacter))
  (bind _output_get (set `/Game/DCT/Blueprints/Core/BP_PlayerCharacter.CharacterSheetRef` _returnvalue (`local.PlayerCharacter`)))
  (`BlueprintMapLibrary.Map_Add` (`self.CharacterSheets`) (`local.PlayerCharacter`) _output_get)
  (`PanelWidget.AddChild` (`/Game/DCT/UserInterface/WBP_Layout.SheetSwitcher` (`self.LayoutRef`)) _output_get)
  (bind _returnvalue_2 (`|CreateWidget` "/Game/DCT/UserInterface/WBP_MiniCharacter.WBP_MiniCharacter_C" self _output_get (`local.PlayerCharacter`)))
  (`UniformGridPanel.AddChildToUniformGrid` (`/Game/DCT/UserInterface/WBP_Layout.MiniCharacterPanel` (`self.LayoutRef`)) _returnvalue_2 (/ _characterindex 2) (mod _characterindex 2))
  (`/Game/DCT/UserInterface/WBP_MiniCharacter.UpdateMiniCharacter` _returnvalue_2)
  (set `/Game/DCT/Blueprints/Core/BP_PlayerCharacter.MiniCharacterRef` _returnvalue_2 (`local.PlayerCharacter`))
  (return))

(fn `UpdateMouseFollowWidgetInViewport`
  (locals (LocalWidgetSize :type "Vector2D Structure" :default (96.0 96.0)))
  (`Widget.RemoveFromParent` (`self.MouseFollowWidget`))
  (`CanvasPanel.AddChildToCanvas` (`/Game/DCT/UserInterface/WBP_Layout.HeldItemCanvas` (`self.LayoutRef`)) (`self.MouseFollowWidget`))
  (`CanvasPanelSlot.SetSize` (`WidgetLayoutLibrary.SlotAsCanvasSlot` (`self.MouseFollowWidget`)) (`local.LocalWidgetSize`))
  (`Widget.SetVisibility` (`self.MouseFollowWidget`) "HitTestInvisible")
  (return))

(fn `UserConstructionScript`)